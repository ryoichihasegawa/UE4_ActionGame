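; Enemy character Blueprint, apparently a wolf, that bites the player and dies when its HP runs out.
; BiteAttack turns toward the player and pulses the anim flag; a toggleable collision detects hits.
; Hits spawn Niagara impact effects and send damage to the player's HP bar, but pass zero to the HP decrement.
; Tick positions the viewport HP widget and, at zero HP, stops AI logic, plays death and destroys the actor.
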(event OnComponentBeginOverlap(BiteAttackCollision)
  (params (OverlappedComponent :type Primitive%20Component%20Object%20Reference) (OtherActor :type Actor%20Object%20Reference) (OtherComp :type Primitive%20Component%20Object%20Reference) (OtherBodyIndex :type Integer) (bFromSweep :type Boolean) (SweepResult :type Hit%20Result%20Structure%20%28by%20ref%29))
  (bind _player_001 (Variables|Default|GetPlayer%20001))
  (if (== OtherActor _player_001)
    (Default|OnDamageEvent self _player_001 (Utilities|Struct|MakeS_DamageParamater 2.0))
    (Development|PrintString "wolfhit")))

(event Custom|BiteAttack
  (bind _returnvalue (Transformation|GetActorLocation))
  (bind _player_001 (Variables|Default|GetPlayer%20001))
  (bind _anim (Variables|Default|GetAnim))
  (bind _returnvalue_2 (Transformation|GetActorLocation _player_001))
  (bind _returnvalue_3 (Math|Rotator|FindLookatRotation _returnvalue _returnvalue_2))
  (Transformation|SetActorRotation (Math|Rotator|MakeRotator (.roll _returnvalue_3) 0.0 (.yaw _returnvalue_3)))
  (Variables|/Game/Blueprints/Character/Enemy/Enemy_001/Anim_Enemy_001/AB_Enemy_001.AB_Enemy_001_C|SetAttackFlag _anim true)
  (Utilities|FlowControl|Delay 0.83)
  (Variables|/Game/Blueprints/Character/Enemy/Enemy_001/Anim_Enemy_001/AB_Enemy_001.AB_Enemy_001_C|SetAttackFlag _anim false))

(event EventBeginPlay
  (|CallParentFunction)
  ;[1 1 1] Anim変数の設定
  (bind _asab_enemy_001 (Utilities|Casting|CastToAB_Enemy_001 (Components|SkeletalMesh|GetAnimInstance (Variables|Character|GetMesh))))
  (Variables|Default|SetAnim _asab_enemy_001)
  ;[1 1 1] Player変数
  (bind _asbp_player_001 (Utilities|Casting|CastToBP_Player_001 (Game|GetPlayerCharacter 0)))
  (Variables|Default|SetPlayer%20001 _asbp_player_001)
  (bind _returnvalue (UserInterface|CreateWidget "/Game/Blueprints/Character/Enemy/Enemy_001/WBP_Enemy_001_HPBar.WBP_Enemy_001_HPBar_C" 0 (Variables|Default|GetEnemy_001HP)))
  (bind _output_get (Variables|Default|SetEnemy_001_HPBar _returnvalue))
  (UserInterface|Viewport|AddtoViewport _output_get 0))

(event Collision|EventActorBeginOverlap
  (params (OtherActor :type Actor%20Object%20Reference))
  (|CallParentFunction OtherActor) ; このノードは無効になっているため呼び出せません。\n機能をビルドするにはピンをドラッグしてください。
)

(event EventTick
  (params (DeltaSeconds :type Float%20%28single-precision%29))
  ;[1 1 1] 常に処理をする
  (|CallParentFunction DeltaSeconds)
  (Utilities|FlowControl|Sequence
    (:then_0
      ;[1 1 1] HPバーの設定
      (bind _enemy_001_hpbar (Variables|Default|GetEnemy_001_HPBar)
        (:then
          (Default|UpdateUILocation _enemy_001_hpbar (Transformation|GetWorldLocation (Variables|Default|GetUIPos))))
        (:else)))
    (:then_1
      (if (<= (Variables|Default|GetEnemy_001HP) 0.0)
        (AI|Logic|StopLogic (Variables|/Script/AIModule.AIController|GetBrainComponent (AI|GetAIController self)) "")
        (Variables|/Game/Blueprints/Character/Enemy/Enemy_001/Anim_Enemy_001/AB_Enemy_001.AB_Enemy_001_C|SetIsDeath? (Variables|Default|GetAnim) true)
        (Utilities|FlowControl|Delay 2.07)
        (Variables|/Game/Blueprints/Character/Enemy/Enemy_001/Anim_Enemy_001/AB_Enemy_001.AB_Enemy_001_C|SetIsDeath? (Variables|Default|GetAnim) false)
        (Actor|DestroyActor)))))

(event EventDisableDamageCollision
  (Collision|SetCollisionEnabled (Variables|Default|GetBiteAttackCollision) "NoCollision"))

(event EventEnableDamageCollision
  (Collision|SetCollisionEnabled (Variables|Default|GetBiteAttackCollision) "QueryAndPhysics"))

(event EventOnDamageEvent
  (params (inOtherActor :type Actor%20Object%20Reference) (inDamageParam :type S%20Damage%20Paramater%20Structure))
  (bind _asbp_player_001 (Utilities|Casting|CastToBP_Player_001 inOtherActor))
  (Niagara|SpawnSystematLocation "/Game/Hack_And_Slash_FX/VFX_Niagara/Impacts/NS_Claws_Impact.NS_Claws_Impact" (Transformation|GetActorLocation _asbp_player_001))
  (CallFunction|PlayerDecreaceHP _asbp_player_001 0.0)
  (Default|OnTakeDamage (Variables|/Game/Blueprints/Character/Character/Player_001/BP_Player_001.BP_Player_001_C|GetPlayerHPBar _asbp_player_001) (.damagevalue inDamageParam)))

(fn ConstructionScript
  (|CallParentFunction))

(fn PlayerDecreaceHP
  (params (Player%20Actor :type Actor%20Object%20Reference) (DamageValue :type Float%20%28single-precision%29))
  (bind _asbp_player_001 (Utilities|Casting|CastToBP_Player_001 Player%20Actor))
  (bind _output_get (Variables|/Game/Blueprints/Character/Character/Player_001/BP_Player_001.BP_Player_001_C|SetPlayer_HP%20 _asbp_player_001 (- (Variables|/Game/Blueprints/Character/Character/Player_001/BP_Player_001.BP_Player_001_C|GetPlayer_HP%20 _asbp_player_001) DamageValue)))
  (return _output_get))

(fn RemoveWiget
  (Widget|RemovefromParent (Variables|Default|GetEnemy_001_HPBar)))