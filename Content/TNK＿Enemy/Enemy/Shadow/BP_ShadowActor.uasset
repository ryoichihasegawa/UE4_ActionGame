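; BP_ShadowActor is a short-lived shadow actor, filed under enemies, that fades out its skeletal mesh like an afterimage.
; BeginPlay records the spawn time and destroys the actor after the DestryTime delay.
; Tick creates a new MI_Shadow dynamic material instance on the mesh's first slot every frame, lowering its "Opa" parameter linearly with elapsed time.
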(event EventBeginPlay
  (Variables|Default|SetTime (Utilities|Time|GetGameTimeinSeconds))
  (Utilities|FlowControl|Delay (Variables|Default|GetDestryTime))
  (Actor|DestroyActor))

(event EventTick
  (params (DeltaSeconds :type Float%20%28single-precision%29))
  (bind _returnvalue (Rendering|Material|CreateDynamicMaterialInstance (Variables|Default|GetSkeletalMesh) 0 "/Game/TNK＿Enemy/Enemy/Shadow/MI_Shadow.MI_Shadow" "None" :!class /Script/Engine.PrimitiveComponent))
  (bind _output_get (Variables|Default|SetShadowMaterial _returnvalue))
  (Rendering|Material|SetScalarParameterValue _output_get "Opa" (- 0.3 (- (Utilities|Time|GetGameTimeinSeconds) (Variables|Default|GetTime))) :!class /Script/Engine.MaterialInstanceDynamic))

(fn ConstructionScript)