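; Sword enemy character that feeds perception results and player state to its AI controller and provides combat actions.
; Each tick it forwards the player's attack flag to the controller.
; AI perception updates target and line-of-sight keys when the player is seen, and uses a timer event for clearing a lost target.
; Events play attack, guard and randomized avoidance montages, and a function sets walk speed.
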(event OnTargetPerceptionUpdated(AIPerception)
  (params (Actor :type Actor%20Object%20Reference) (Stimulus :type AI%20Stimulus%20Structure))
  (bind _aicontroller (Variables|Default|GetAIController))
  ;[1 1 1] AIPerception(視覚)
  (bind _output_get (Variables|Default|SetPerceivedActor Actor))
  (if (and (== _output_get (Variables|Default|GetPlayerCharacter)) (Utilities|Struct|BreakAIStimulus Stimulus))
    (Variables|Default|SetPerceivedActor (Variables|Default|GetPlayerCharacter))
    (Utilities|Time|ClearandInvalidateTimerbyHandle (Variables|Default|GetTagetLostTime))
    (Class|BPEnemyAIConInterface|UpdateTagetActorKey(Message) _aicontroller (Variables|Default|GetPerceivedActor))
    (Class|BPEnemyAIConInterface|UpdateHasLineOfSightKey(Message) _aicontroller true)
    (elif (== (Variables|Default|GetPerceivedActor) (Variables|Default|GetPlayerCharacter))
      (bind _returnvalue (Utilities|Time|SetTimerbyEvent (delegate Custom|TagetLost) 0.0))
      (Variables|Default|SetTagetLostTime _returnvalue)
      (Class|BPEnemyAIConInterface|UpdateHasLineOfSightKey(Message) _aicontroller false))))

(event Custom|TagetLost
  ;[1 1 1] AIPerception(視覚)
  (Class|BPEnemyAIConInterface|UpdateTagetActorKey(Message) (Variables|Default|GetAIController)))

(event EventBeginPlay
  ;[1 1 1] 始まった瞬間にプレイヤーの変数を入れる
  (Variables|Default|SetPlayerCharacter (Game|GetPlayerCharacter 0))
  (Variables|Default|SetAIController (Pawn|GetController)))

(event EventAvoidance
  ;[1 1 1] 回避
  (Animation|Montage|PlayMontage (Variables|Character|GetMesh) "/Game/TNK＿Enemy/Enemy/Animation/AnimationMontage/AM_Avoidance.AM_Avoidance" 1.0 0.0 (Utilities|Array|Get(acopy) (Variables|Default|GetAnim_AvoidanceNameList) (Math|Random|RandomInteger 3))))

(event EventAttack
  ;[1 1 1] 攻撃
  (Animation|Montage|PlayMontage (Variables|Character|GetMesh) "/Game/TNK＿Enemy/Enemy/Animation/AnimationMontage/AM_Attack.AM_Attack"))

(event EventTick
  (params (DeltaSeconds :type Float%20%28single-precision%29))
  (bind _asplayer_pawn (Utilities|Casting|CastToPlayer_Pawn (Variables|Default|GetPlayerCharacter)))
  (Class|BPEnemyAIConInterface|UpdatePlayerAttackFlagKey(Message) (Variables|Default|GetAIController) (Variables|/Game/Player/Blueprint/Player_Pawn.Player_Pawn_C|GetAttack_frag _asplayer_pawn)))

(event EventGuard
  ;[1 1 1] ガード
  (Animation|Montage|PlayMontage (Variables|Character|GetMesh) 0))

(fn ConstructionScript)

(fn UpdateWalkSpeed
  (params (NewWalkSpeed :type Float%20%28single-precision%29))
  (Variables|/Script/Engine.CharacterMovementComponent|SetMaxWalkSpeed (Variables|Character|GetCharacterMovement) NewWalkSpeed))