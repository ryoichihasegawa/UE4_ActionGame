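; BP_TrackingMagic is an enemy magic projectile that homes in on the player for a limited time.
; On BeginPlay it casts player character 0 to Player_Pawn and sets that pawn's root component as the ProjectileMovement homing target.
; Tick lowers HomingTime by one per frame, independent of delta time, and switches homing off once it reaches zero.
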(event EventBeginPlay
  (|CallParentFunction)
  (bind _asplayer_pawn (Utilities|Casting|CastToPlayer_Pawn (Game|GetPlayerCharacter 0)))
  (bind _output_get (Variables|Default|SetAs%20Player%20Pawn _asplayer_pawn))
  (Variables|/Script/Engine.ProjectileMovementComponent|SetHomingTargetComponent (Variables|Default|GetProjectileMovement) (Variables|/Script/Engine.Actor|GetRootComponent _output_get)))

(event EventTick
  (params (DeltaSeconds :type Float%20%28single-precision%29))
  (bind _projectilemovement (Variables|Default|GetProjectileMovement))
  (bind _output_get (Variables|Default|SetHoming%20Time (- (Variables|Default|GetHoming%20Time) 1.0)))
  (if (<= _output_get 0.0)
    (if (Variables|/Script/Engine.ProjectileMovementComponent|GetbIsHomingProjectile _projectilemovement)
      (Variables|/Script/Engine.ProjectileMovementComponent|SetbIsHomingProjectile _projectilemovement false))))

(fn ConstructionScript
  (|CallParentFunction))