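; BP_HitEnemyContext is an EQS query context that supplies a single location taken from objects near the querier.
; It runs a multi sphere trace from the querier actor's location along an offset, filtered by a desired object type.
; It returns the location of a randomly chosen hit, with no check for an empty result.
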(fn ProvideSingleLocation
  (params (QuerierObject :type Object%20Object%20Reference) (QuerierActor :type Actor%20Object%20Reference))
  (bind _returnvalue (Transformation|GetActorLocation QuerierActor))
  (bind _outhits (Collision|MultiSphereTraceForObjects _returnvalue (+ _returnvalue (Variables|Default|GetDffset)) 0.0 (Variables|Default|GetDesiredObjectType) false 0 "None"))
  (return (.Location (Collision|BreakHitResult (Utilities|Array|Get(acopy) _outhits (Math|Random|RandomIntegerinRange 0 (- (Utilities|Array|Length _outhits) 1)))))))