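; Base wizard enemy character that hunts the player with aimed magic shots and particle-marked warps, ragdolling on death.
; Sight perception sets the AI target, plays a discovery montage and alerts actors sharing its tag; a timer clears the target after sight loss.
; Tick pushes cooldowns, chance values, the player's attack flag and a line-trace attack flag to the AI controller through key-update messages.
; Taking a hit while alive also targets the player.
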(event OnTargetPerceptionUpdated(AIPerception)
  (params (Actor :type Actor%20Object%20Reference) (Stimulus :type AI%20Stimulus%20Structure))
  (bind _ai_controller (Variables|アクタ|GetAI%20Controller))
  (bind _ai_controller_2 (Variables|アクタ|GetAI%20Controller))
  (bind _braincomponent (Variables|/Script/AIModule.AIController|GetBrainComponent _ai_controller_2))
  ;[0 1 0] AIPerception
  (Variables|アクタ|SetPerceivedActor Actor)
  (if (and (== (Variables|アクタ|GetPerceivedActor) (Variables|アクタ|GetPlayerCharacter)) (Utilities|Struct|BreakAIStimulus Stimulus)) ; 視界にいるか？
    (Variables|アクタ|SetPerceivedActor (Variables|アクタ|GetPlayerCharacter))
    (Utilities|FlowControl|Sequence
      (:then_0
        (Utilities|Time|ClearandInvalidateTimerbyHandle (Variables|ＡＩ|GetTagetLostTime))
        (Class|BPEnemyAIConInterface|UpdateTagetActorKey(Message) _ai_controller (Variables|アクタ|GetPerceivedActor))
        (Class|BPEnemyAIConInterface|UpdateHasLineOfSightKey(Message) _ai_controller true)
        (Utilities|FlowControl|DoOnce false
          (:Completed
            (AI|Logic|StopLogic _braincomponent "")
            (Animation|Montage|PlayMontage (Variables|Character|GetMesh) "/Game/TNK＿Enemy/Enemy/Animation/AnimationMontage/Corpse/AM_EnemyDiscover.AM_EnemyDiscover"
              (:then
                (Utilities|FlowControl|Delay 1.0)
                (Class|BrainComponent|RestartLogic _braincomponent))))))
      (:then_1
        (bind _outactors (Actor|GetAllActorswithTag (Utilities|Array|Get(acopy) (Variables|Default|GetTags) 1)))
        (for _array_element _outactors
          (Class|BPEnemyAIConInterface|UpdateTagetActorKey(Message) (AI|GetAIController _array_element) (Variables|アクタ|GetPerceivedActor)))))
    (elif (== (Variables|アクタ|GetPlayerCharacter) (Variables|アクタ|GetPerceivedActor)) ; 視界から外れた処理
      (bind _returnvalue (Utilities|Time|SetTimerbyEvent (delegate Custom|TagetLost) 5.0))
      (Variables|ＡＩ|SetTagetLostTime _returnvalue)
      (Class|BPEnemyAIConInterface|UpdateHasLineOfSightKey(Message) (Variables|アクタ|GetAI%20Controller) false)
      (AI|ClearFocus (Variables|アクタ|GetAI%20Controller)))))

(event Custom|Shot
  ;[1 1 1] 攻撃
  ;;[0 0 0.979] 弾の処理
  (Game|SpawnActorfromClass (Variables|攻撃|GetMagic) (Math|Transform|MakeTransform (Transformation|GetSocketLocation (Variables|Character|GetMesh) "Bip001-Spine1") (Math|Rotator|FindLookatRotation (Transformation|GetActorLocation) (Transformation|GetActorLocation (Variables|アクタ|GetPlayerCharacter))) "1,1,1") "Undefined" 0 0) ; 弾
)

(event Custom|TagetLost
  (bind _ai_controller (Variables|アクタ|GetAI%20Controller))
  (bind _braincomponent (Variables|/Script/AIModule.AIController|GetBrainComponent _ai_controller))
  ;[0 1 0] AIPerception
  (Class|BPEnemyAIConInterface|UpdateTagetActorKey(Message) (Variables|アクタ|GetAI%20Controller))
  (AI|Components|Blackboard|SetValueasBool (AI|GetBlackboard self) (Variables|ＡＩ|GetMoveSuccessName) false)
  (AI|ClearFocus (Variables|アクタ|GetAI%20Controller))
  (Utilities|FlowControl|DoOnce false) ; enters at Reset
)

(event EventBeginPlay
  (CallFunction|EnemyBegin self))

(event EventSetAttackCoolDownTime
  ;[1 1 1] 攻撃
  ;;[0 1 0] クールダウン時間を更新
  (Class|BPEnemyAIConInterface|UpdateAttackCoolDownTimeKey(Message) (Variables|アクタ|GetAI%20Controller) (Variables|攻撃|GetAttack%20Cool%20Down%20Time)))

(event EventAttack
  ;[1 1 1] 攻撃
  ;;[1 0 0] 攻撃イベント呼び出し
  (Animation|PlayAnimMontage "/Game/TNK＿Enemy/Enemy/Animation/AnimationMontage/Corpse/AM_EnemyWizardAttack.AM_EnemyWizardAttack" 1.0 "None")
  (Variables|攻撃|SetAttack%20Cool%20Down%20Time (Variables|攻撃|GetAttack%20Cool%20Down%20Initial%20Time)))

(event EventTick
  (params (DeltaSeconds :type Float%20%28single-precision%29))
  (bind _ai_controller (Variables|アクタ|GetAI%20Controller))
  ;[1 1 1] 常にやる
  (bind _output_get (Variables|Default|SetTime DeltaSeconds))
  (|CallParentFunction _output_get)
  (Utilities|FlowControl|Sequence
    (:then_0
      (ＡＩ|UpdateKey (.AsPlayer%20Pawn (Utilities|Casting|CastToPlayer_Pawn (Variables|アクタ|GetPlayerCharacter)))) ; Keyのまとめ
    )
    (:then_1
      (ＡＩ|UpdateEnemyAttackFlag) ; EnemyAttackFlagを更新する
    )
    (:then_2
      (Utilities|FlowControl|Sequence
        (:then_0
          ;;[0 0 1] CoolDownTime処理
          (if (>= (Variables|攻撃|GetAttack%20Cool%20Down%20Time) 0.0)
            (bind _output_get_2 (Variables|攻撃|SetAttack%20Cool%20Down%20Time (- (Variables|攻撃|GetAttack%20Cool%20Down%20Time) (Variables|Default|GetTime))))
            (Class|BPEnemyAIConInterface|UpdateAttackCoolDownTimeKey(Message) _ai_controller _output_get_2)))
        (:then_1
          (if (>= (Variables|移動|GetWarp%20Cool%20Down%20Time) 0.0)
            (bind _output_get_3 (Variables|移動|SetWarp%20Cool%20Down%20Time (- (Variables|移動|GetWarp%20Cool%20Down%20Time) (Variables|Default|GetTime))))
            (Class|BPEnemyAIConInterface|UpdateWarpCoolDownTimeKey(Message) _ai_controller _output_get_3)))))))

(event EventOnEnemyDamageEvent
  (params (In_Other_Actor :type Actor%20Object%20Reference) (Damage_Parameter :type Damage%20Parameter%20Structure))
  ;[1 1 1] ダメージ処理
  ;;[1 0 0] ダメージ食らった時の処理
  (|CallParentFunction In_Other_Actor Damage_Parameter))

(event EventMove
  (params (Location :type Vector :default "0, 0, 0"))
  (bind (_x _y _z) (Math|Vector|BreakVector Location))
  (bind (_x_2 _y_2) (Math|Vector|BreakVector Location))
  (bind _warp_move_particle_ (Variables|移動|GetWarp%20Move%20Particle%20))
  ;[1 1 1] ワープ移動
  (bind _returnvalue (Effects|SpawnEmitteratLocation (Variables|Particle|GetWarp%20MoveEmitter%20Template) (Transformation|GetSocketLocation (Variables|Character|GetMesh) "ROOT") "0, 0, 0" "0.500000,0.500000,0.500000"))
  (Utilities|Array|Add (Variables|移動|GetWarp%20Move%20Particle%20) _returnvalue)
  (Timeline|MoveTime PlayFromStart
    (:Finished
      (bind _returnvalue_2 (Effects|SpawnEmitteratLocation (Variables|Particle|GetWarp%20MoveEmitter%20Template) (Math|Vector|MakeVector _x_2 _y_2 (.z (Transformation|GetSocketLocation (Variables|Character|GetMesh) "ROOT"))) "0, 0, 0" "0.500000,0.500000,0.500000"))
      (Utilities|Array|Add (Variables|移動|GetWarp%20Move%20Particle%20) _returnvalue_2)
      (Utilities|FlowControl|Delay 0.6)
      (Transformation|SetActorLocation (Math|Vector|MakeVector _x _y (+ _z 1.5e+02)) false false)
      (Variables|移動|SetWarp%20Cool%20Down%20Time (Variables|移動|GetWarp%20Cool%20Down%20Initial%20Time))
      (Components|DestroyComponent _warp_move_particle_)
      (Utilities|Array|Clear _warp_move_particle_)
      (Default|SetWarpCoolDownTime self))))

(event EventEndPlay
  (params (EndPlayReason :type EEndPlayReason%20Enum :default "Destroyed"))
  (bind _warp_move_particle_ (Variables|移動|GetWarp%20Move%20Particle%20))
  (|CallParentFunction EndPlayReason)
  (Components|DestroyComponent _warp_move_particle_)
  (Utilities|Array|Clear _warp_move_particle_))

(event EventSetWarpCoolDownTime
  ;[1 1 1] ワープ移動
  (Class|BPEnemyAIConInterface|UpdateWarpCoolDownTimeKey(Message) (Variables|アクタ|GetAI%20Controller) (Variables|移動|GetWarp%20Cool%20Down%20Time)))

(event EventHitAnimation
  (bind _ai_controller (Variables|アクタ|GetAI%20Controller))
  ;[1 1 1] ダメージ処理
  ;;[0 1 0] 当たった時の処理
  (Animation|PlayAnimMontage "/Game/TNK＿Enemy/Enemy/Animation/AnimationMontage/Corpse/AM_EnemyDamage.AM_EnemyDamage" 1.0 "None")
  (Audio|PlaySound2D "/Game/TNK＿Enemy/Enemy/Sound/Damage/SC_Damage.SC_Damage" 1.0 1.0 0.0 0 0)
  (bind _return (Class|BPEnemyInterface|IsAlive(Message) self))
  (if _return
    (AI|SetFocus _ai_controller (Variables|アクタ|GetPlayerCharacter))
    (Variables|アクタ|SetPerceivedActor (Variables|アクタ|GetPlayerCharacter))
    (Class|BPEnemyAIConInterface|UpdateTagetActorKey(Message) (Variables|アクタ|GetAI%20Controller) (Variables|アクタ|GetPlayerCharacter))
    (else
      (AI|ClearFocus _ai_controller))))

(event EventDeadAnimation
  (bind _mesh (Variables|Character|GetMesh))
  ;[1 1 1] ダメージ処理
  ;;[1 0 0.8039] 死亡処理
  (Audio|PlaySound2D "/Game/TNK＿Enemy/Enemy/Sound/Death/SC_Death.SC_Death" 1.0 1.0 0.0 0 0)
  (Class|SkeletalMeshComponent|SetAllBodiesSimulatePhysics _mesh true)
  (Collision|SetCollisionEnabled _mesh "PhysicsOnly"))

(fn ConstructionScript
  (|CallParentFunction))

(fn UpdateWalkSpeed
  (params (NewWalkSpeed :type Float%20%28single-precision%29))
  (Variables|/Script/Engine.CharacterMovementComponent|SetMaxWalkSpeed (Variables|Character|GetCharacterMovement) NewWalkSpeed))

(fn UpdateEnemyAttackFlag
  (bind _mesh (Variables|Character|GetMesh))
  (bind _returnvalue (Transformation|GetSocketLocation _mesh "Bip001-Spine1"))
  (if (ScalableFloat|GetValueasBool (AI|GetBlackboard 0) (Variables|ＡＩ|GetMoveSuccessName))
    (bind _outhit (Collision|LineTraceByChannel _returnvalue (+ _returnvalue (* (Math|Vector|GetForwardVector (Math|Rotator|FindLookatRotation (Transformation|GetActorLocation) (Transformation|GetActorLocation (Variables|アクタ|GetPlayerCharacter)))) 2.5e+03)) "TraceTypeQuery1" false 0 "None"))
    (if (== (Variables|アクタ|GetPlayerCharacter) (.HitActor (Collision|BreakHitResult _outhit)))
      (Variables|攻撃|SetEnemyAttackFlag true)
      (else
        (Variables|攻撃|SetEnemyAttackFlag false)))))

(fn UpdateKey
  (params (Player%20Pawn :type Player%20Pawn%20Object%20Reference))
  ;[1 1 1] 常にプレイヤーのAttackFragを更新する
  (Class|BPEnemyAIConInterface|UpdatePlayerAttackFlagKey(Message) (Variables|アクタ|GetAI%20Controller) (Variables|/Game/Player/Blueprint/Player_Pawn.Player_Pawn_C|GetAttack_frag Player%20Pawn))
  ;[1 1 1] 常にEnemyAttackFlagを更新する
  (Class|BPEnemyAIConInterface|UpdateEnemyAttackFlagKey(Message) (Variables|アクタ|GetAI%20Controller) (Variables|攻撃|GetEnemyAttackFlag))
  ;[1 1 1] 攻撃の確率の値を更新
  (Class|BPEnemyAIConInterface|UpdateAttackRandomKey(Message) (Variables|アクタ|GetAI%20Controller) (Variables|ＡＩ|GetAttackRandam))
  ;[1 1 1] ワープする確率の値を更新
  (Class|BPEnemyAIConInterface|UpdateWarpRandamKey(Message) (Variables|アクタ|GetAI%20Controller) (Variables|ＡＩ|GetWarpRandam)))

(fn EnemyBegin
  (|CallParentFunction)
  ;[1 1 1] 始まった瞬間に格納
  (Variables|アクタ|SetPlayerCharacter (Game|GetPlayerCharacter 0))
  (Variables|アクタ|SetAI%20Controller (AI|GetAIController self))
  ;[1 1 1] 初期値を格納
  (Variables|移動|SetWarp%20Cool%20Down%20Initial%20Time (Variables|移動|GetWarp%20Cool%20Down%20Time))
  (Variables|攻撃|SetAttack%20Cool%20Down%20Initial%20Time (Variables|攻撃|GetAttack%20Cool%20Down%20Time))
  ;[1 1 1] 始まったら更新する
  (Class|BPEnemyAIConInterface|UpdateAttackCoolDownTimeKey(Message) (Variables|アクタ|GetAI%20Controller) 0.0)
  (Class|BPEnemyAIConInterface|UpdateWarpCoolDownTimeKey(Message) (Variables|アクタ|GetAI%20Controller) 0.0))

(fn IsAlive
  (return (> (Variables|Default|GetHP) 0.0)))