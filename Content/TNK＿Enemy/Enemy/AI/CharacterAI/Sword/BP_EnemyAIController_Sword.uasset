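; AI controller for sword-wielding enemies that runs the BT_Enemy_Sword behavior tree on BeginPlay.
; A set of update events writes values into the Blackboard under named keys: player and target actors, line of sight, random attack and avoidance values, player-attack and parry-success flags.
; The controller makes no decisions itself, only relaying incoming state to the Blackboard.
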(event EventBeginPlay
  (AI|RunBehaviorTree "/Game/TNK＿Enemy/Enemy/AI/CharacterAI/Sword/BT_Enemy_Sword.BT_Enemy_Sword"))

(event EventUpdateHasLineOfSightKey
  (params (HasLineOfSight :type Boolean))
  ;[1 1 1] Has line of sight keyをブラックボードに取得
  (AI|Components|Blackboard|SetValueasBool (Variables|Default|GetBlackboard) (Variables|Default|GetHasLineOfSightName) HasLineOfSight))

(event EventUpdatePlayerAttackFlagKey
  (params (PlayerAttackFlag :type Boolean))
  ;[1 1 1] PlayerAttackFlagをブラックボードに取得
  (AI|Components|Blackboard|SetValueasBool (Variables|Default|GetBlackboard) (Variables|Default|GetPlayerAttackFlagName) PlayerAttackFlag))

(event EventUpdateParrySuccessFlagKey
  (params (ParrySuccessFlag :type Boolean))
  ;[1 1 1] ParrySuccessFlagをブラックボードに取得
  (AI|Components|Blackboard|SetValueasBool (Variables|Default|GetBlackboard) (Variables|Default|GetParrySuccessFlagName) ParrySuccessFlag))

(event EventUpdateTagetActorKey
  (params (TagetActor :type Actor%20Object%20Reference))
  ;[1 1 1] Taget Actorをブラックボードに取得
  (AI|Components|Blackboard|SetValueasObject (Variables|Default|GetBlackboard) (Variables|Default|GetTagetActorName) TagetActor))

(event EventUpdateAvoidanceRandamKey
  (params (AvoidanceRandam :type Float%20%28single-precision%29))
  ;[1 1 1] AvoidanceRandamをブラックボードに取得
  (AI|Components|Blackboard|SetValueasFloat (Variables|Default|GetBlackboard) (Variables|Default|GetAvoidanceRandamName) AvoidanceRandam))

(event EventUpdateAttackRandomKey
  (params (AttackRandam :type Float%20%28single-precision%29))
  ;[1 1 1] AttackRandamをブラックボードに取得
  (AI|Components|Blackboard|SetValueasFloat (Variables|Default|GetBlackboard) (Variables|Default|GetAttackRandamName) AttackRandam))

(event EventUpdatePlayerActorKey
  (params (PlayerActor :type Actor%20Object%20Reference))
  ;[1 1 1] Player Actorをブラックボードに取得
  (AI|Components|Blackboard|SetValueasObject (Variables|Default|GetBlackboard) (Variables|Default|GetPlayer%20Actor%20Name) PlayerActor))

(fn ConstructionScript)