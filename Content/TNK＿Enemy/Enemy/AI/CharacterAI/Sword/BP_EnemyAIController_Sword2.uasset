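; AI controller for the sword enemy character, driving its behavior through a behavior tree.
; On BeginPlay it runs BT_Enemy_Sword.
; Custom events write the target actor, line-of-sight flag and player attack flag into named Blackboard keys for the tree to read.
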(event EventBeginPlay
  (AI|RunBehaviorTree "/Game/TNK＿Enemy/Enemy/AI/CharacterAI/Sword/BT_Enemy_Sword.BT_Enemy_Sword"))

(event EventUpdateHasLineOfSightKey
  (params (HasLineOfSight :type Boolean))
  ;[1 1 1] Has line of sight keyをブラックボードに取得
  (AI|Components|Blackboard|SetValueasBool (Variables|Default|GetBlackboard) (Variables|Default|GetHasLineOfSightName) HasLineOfSight))

(event EventUpdatePlayerAttackFlagKey
  (params (PlayerAttackFlag :type Boolean))
  ;[1 1 1] PlayerAttackFlagをブラックボードに取得
  (AI|Components|Blackboard|SetValueasBool (Variables|Default|GetBlackboard) (Variables|Default|GetPlayerAttackFlagName) PlayerAttackFlag))

(event EventUpdateTagetActorKey
  (params (TagetActor :type Actor%20Object%20Reference))
  ;[1 1 1] Taget Actorをブラックボードに取得
  (AI|Components|Blackboard|SetValueasObject (Variables|Default|GetBlackboard) (Variables|Default|GetTagetActorName) TagetActor))

(fn ConstructionScript)