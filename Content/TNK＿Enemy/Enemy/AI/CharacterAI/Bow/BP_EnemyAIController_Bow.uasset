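; AI controller for the bow-wielding enemy, running the BT_Enemy_Bow behavior tree on BeginPlay.
; Custom events write state into Blackboard keys: the target actor, line of sight, bow possession and the attack flag.
; Each key name comes from a variable, and the controller itself holds no decision logic beyond these setters.
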(event EventBeginPlay
  (AI|RunBehaviorTree "/Game/TNK＿Enemy/Enemy/AI/CharacterAI/Bow/BT_Enemy_Bow.BT_Enemy_Bow"))

(event EventUpdateHasLineOfSightKey
  (params (HasLineOfSight :type Boolean))
  ;[1 1 1] Has Line Of Sight Keyをブラックボードに取得
  (AI|Components|Blackboard|SetValueasBool (Variables|Default|GetBlackboard) (Variables|KeyName|GetHasLineOfSightName) HasLineOfSight))

(event EventUpdateHasBowKey
  (params (HasBow :type Boolean))
  ;[1 1 1] Has Bow Key をブラックボードに取得
  (AI|Components|Blackboard|SetValueasBool (Variables|Default|GetBlackboard) (Variables|KeyName|GetHasBowName) HasBow))

(event EventUpdateEnemyAttackFlagKey
  (params (EnemyAttackFlag :type Boolean))
  ;[1 1 1] Has Bow Key をブラックボードに取得
  (AI|Components|Blackboard|SetValueasBool (Variables|Default|GetBlackboard) (Variables|KeyName|GetEnemyAttackFlagName) EnemyAttackFlag))

(event EventUpdateTagetActorKey
  (params (TagetActor :type Actor%20Object%20Reference))
  ;[1 1 1] Taget Actor Keyをブラックボードに取得
  (AI|Components|Blackboard|SetValueasObject (Variables|Default|GetBlackboard) (Variables|KeyName|GetTagetActorName) TagetActor))

(fn ConstructionScript)