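; Base Blueprint for sword enemy characters, covering player detection, melee attacks, backward dodges, parry stagger, super armor and ragdoll death.
; Tick feeds flags and cooldowns to the AI controller as keys; sighting the player alerts tagged allies, with delayed target loss.
; Attack picks montages by player distance, using a timeline lunge at mid range.
; Lunges and dodges spawn afterimage actors every frame from pose snapshots.
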(event OnTargetPerceptionUpdated(AIPerception)
  (params (Actor :type Actor%20Object%20Reference) (Stimulus :type AI%20Stimulus%20Structure))
  ;[1 1 1] AIPerception
  (Variables|Actor|SetPerceivedActor Actor)
  (Utilities|FlowControl|Sequence
    (:then_0
      (if (and (== (Variables|Actor|GetPerceivedActor) (Variables|Actor|GetPlayerCharacter)) (Utilities|Struct|BreakAIStimulus Stimulus))
        (Variables|Actor|SetPerceivedActor (Variables|Actor|GetPlayerCharacter))
        (bind _outactors (Actor|GetAllActorswithTag (Utilities|Array|Get(acopy) (Variables|Default|GetTags) 1)))
        (for _array_element _outactors
          (Utilities|Time|ClearandInvalidateTimerbyHandle (Variables|AI|GetTagetLostTime))
          (Class|BPEnemyAIConInterface|UpdateTagetActorKey(Message) (AI|GetAIController _array_element) (Variables|Actor|GetPerceivedActor))
          (Class|BPEnemyAIConInterface|UpdateHasLineOfSightKey(Message) (Variables|Actor|GetAIController) true)
          (CallFunction|UpdateWalkSpeed (Variables|移動|GetDiscoverWalk%20Speed)) ; WalkSpeedを更新
          (Utilities|FlowControl|DoOnce false
            (:Completed
              (AI|Logic|StopLogic (Variables|Default|GetBrain%20Component) "")
              (Animation|Montage|PlayMontage (Variables|Character|GetMesh) (Variables|Default|GetDiscoverAnim%20Montage)
                (:OnCompleted
                  (Class|BrainComponent|RestartLogic (Variables|Default|GetBrain%20Component)))))))
        (elif (== (Variables|Actor|GetPlayerCharacter) (Variables|Actor|GetPerceivedActor))
          (bind _returnvalue (Utilities|Time|SetTimerbyEvent (delegate Custom|TagetLost) 5.0))
          (Variables|AI|SetTagetLostTime _returnvalue)
          (Class|BPEnemyAIConInterface|UpdateHasLineOfSightKey(Message) (Variables|Actor|GetAIController) false)
          (AI|ClearFocus (Variables|Actor|GetAIController)) ; 見続けるのをやめる
        )))))

(event Custom|Parry
  ;[1 1 1] パリィ処理
  (Variables|パリィ|SetParrySuccessFlag true)
  (AI|Logic|StopLogic (Variables|Default|GetBrain%20Component) "")
  (Collision|SetCollisionEnabled (Variables|Default|GetEnemy_Attack_1) "NoCollision")
  (Animation|StopAnimMontage (Variables|攻撃|GetAttackAnim%20Montage))
  (Animation|Montage|PlayMontage (Variables|Character|GetMesh) (Variables|パリィ|GetParryAnim%20Montage) (Variables|パリィ|GetParry%20Anim%20Play%20Rate)
    (:then
      (Variables|パリィ|SetParyTrueFrag false)
      (Utilities|FlowControl|Delay 3.0)
      (Class|BrainComponent|RestartLogic (Variables|Default|GetBrain%20Component)))
    (:OnCompleted
      (Variables|パリィ|SetParrySuccessFlag false :!label _label))
    (:OnInterrupted
      (goto _label))))

(event Custom|TagetLost
  ;[1 1 1] AIPerception
  (Class|BPEnemyAIConInterface|UpdateTagetActorKey(Message) (Variables|Actor|GetAIController))
  (AI|ClearFocus (Variables|Actor|GetAIController))
  (Utilities|FlowControl|DoOnce false) ; enters at Reset
)

(event EventBeginPlay
  (bind _returnvalue (Pawn|GetController))
  (bind _returnvalue_2 (AI|GetAIController _returnvalue))
  (|CallParentFunction)
  ;[1 1 1] 始まった瞬間に格納
  (Variables|Actor|SetPlayerCharacter (Game|GetPlayerCharacter 0))
  (Variables|Actor|SetAIController _returnvalue_2)
  (Variables|Default|SetBrain%20Component (Variables|/Script/AIModule.AIController|GetBrainComponent _returnvalue_2))
  ;[1 1 1] 初期値を格納
  (Variables|アーマー|SetSuperArmorValue (Variables|アーマー|GetSuperArmorInitial%20Value))
  (Variables|アーマー|SetSuperArmorResetInitialTime (Variables|アーマー|GetSuperArmorResetTime))
  (Variables|攻撃|SetAttack%20Cool%20Down%20Initial%20Time (Variables|攻撃|GetAttack%20Cool%20Down%20Time))
  (Variables|回避|SetAvoidance%20Cool%20Down%20Initial%20Time (Variables|回避|GetAvoidance%20Cool%20Down%20Time))
  ;[1 1 1] 始まったら更新する
  (Class|BPEnemyAIConInterface|UpdatePlayerActorKey(Message) (Variables|Actor|GetAIController) (Variables|Actor|GetPlayerCharacter))
  (Class|BPEnemyAIConInterface|UpdateAttackCoolDownTimeKey(Message) (Variables|Actor|GetAIController) 0.0)
  (Class|BPEnemyAIConInterface|UpdateAvoidanceCoolDownTimeKey(Message) (Variables|Actor|GetAIController) 0.0))

(event EventAvoidance
  ;[1 1 1] 回避処理
  (Variables|回避|SetShadowFlag true)
  (Animation|Montage|PlayMontage (Variables|Character|GetMesh) (Variables|回避|GetAvoidanceAnim%20Montage) (Variables|回避|GetAvoidance%20Anim%20Play%20Rate)
    (:then
      (Timeline|AvoidanceMoveTimeLine PlayFromStart
        (:Update
          (Transformation|SetActorLocation (CallFunction|ForwardMoveto self -15.0) true true)
          (Variables|回避|SetAvoidance%20Cool%20Down%20Time (Variables|回避|GetAvoidance%20Cool%20Down%20Initial%20Time)))))
    (:OnCompleted
      (Variables|回避|SetShadowFlag false :!label _label))
    (:OnInterrupted
      (goto _label))))

(event EventSetAvoidanceCoolDownTime
  ;[1 1 1] 回避処理
  (Class|BPEnemyAIConInterface|UpdateAvoidanceCoolDownTimeKey(Message) (Variables|Actor|GetAIController) (Variables|回避|GetAvoidance%20Cool%20Down%20Time)))

(event EventSetAttackCoolDownTime
  ;[1 1 1] 攻撃処理
  (Class|BPEnemyAIConInterface|UpdateAttackCoolDownTimeKey(Message) (Variables|Actor|GetAIController) (Variables|攻撃|GetAttack%20Cool%20Down%20Time)))

(event EventEnemyDamageDisable
  ;[1 1 1] 攻撃処理
  ;;[1 0.9658 0] 攻撃判定を呼び出し
  (|CallParentFunction)
  (Variables|攻撃|SetEnemyAttack%20Frag false))

(event EventAttack
  (bind _playercharacter (Variables|Actor|GetPlayerCharacter))
  (bind _return (CallFunction|ActorDistance _playercharacter))
  ;[1 1 1] 攻撃処理
  (AI|ClearFocus (Variables|Actor|GetAIController)) ; 見続けるのをやめる
  (if (<= _return 3e+02)
    (if (Variables|Default|GetStrengthEnemyFlag)
      (if (Math|Random|RandomBool)
        (Animation|PlayAnimMontage (Variables|攻撃|GetAttackAnim%20Montage) (Variables|攻撃|GetAttack3%20Play%20Rate) "Anim_Attack3")
        (else
          (Animation|PlayAnimMontage (Variables|攻撃|GetAttackAnim%20Montage) (Variables|攻撃|GetAttack%20Play%20Rate) (Variables|攻撃|GetAM_SectionAttackName) :!label _label)))
      (else
        (goto _label)))
    (Variables|攻撃|SetAttack%20Cool%20Down%20Time (Variables|攻撃|GetAttack%20Cool%20Down%20Initial%20Time) :!label _label_2)
    (elif (<= _return 6e+02)
      (Variables|回避|SetShadowFlag true)
      (Animation|Montage|PlayMontage (Variables|Character|GetMesh) (Variables|攻撃|GetAttackAnim%20Montage) (Variables|攻撃|GetAttack2%20Play%20Rate) 0.0 "Anim_Attack2"
        (:then
          (Timeline|AttackMoveTimeLine PlayFromStart
            (:Update
              (Transformation|SetActorLocation (CallFunction|ForwardMoveto self (Variables|Default|GetMoving%20Distance)) true true)
              (goto _label_2))))
        (:OnCompleted
          _)
        (:OnInterrupted
          _))
      (Variables|回避|SetShadowFlag false)
      (Utilities|FlowControl|Delay (Variables|攻撃|GetAttack2RecastTime)))))

(event EventTick
  (params (DeltaSeconds :type Float%20%28single-precision%29))
  (bind _snapshot (Variables|Default|GetSnapshot))
  ;[1 1 1] 常にやる
  (bind _output_get (Variables|Default|SetTime DeltaSeconds))
  (|CallParentFunction _output_get)
  (bind _asplayer_pawn (Utilities|Casting|CastToPlayer_Pawn (Variables|Actor|GetPlayerCharacter)))
  (Utilities|FlowControl|Sequence
    (:then_0
      (AI|UpdateKey _asplayer_pawn) ; Key更新
    )
    (:then_1
      ;[1 1 1] パリィされた時の処理
      (if (and (Variables|/Game/Player/Blueprint/Player_Pawn.Player_Pawn_C|GetPary_Frag _asplayer_pawn) (Variables|パリィ|GetParyTrueFrag))
        (CallFunction|Parry) ; パリィ
      ))
    (:then_2
      ;[1 1 1] リセット処理
      (if (< (Variables|アーマー|GetSuperArmorValue) (Variables|アーマー|GetSuperArmorInitial%20Value))
        (Variables|アーマー|SetSuperArmorResetTime (- (Variables|アーマー|GetSuperArmorResetTime) (Variables|Default|GetTime)))))
    (:then_3
      ;[1 1 1] アーマーの処理
      (if (and (< (Variables|アーマー|GetSuperArmorValue) (Variables|アーマー|GetSuperArmorInitial%20Value)) (<= (Variables|アーマー|GetSuperArmorResetTime) 0.0))
        (Variables|アーマー|SetSuperArmorValue (Variables|アーマー|GetSuperArmorInitial%20Value))
        (Variables|アーマー|SetSuperArmorResetTime (Variables|アーマー|GetSuperArmorResetInitialTime))))
    (:then_4
      (Utilities|FlowControl|Sequence
        (:then_0
          ;[1 1 1] CoolDownTime処理
          (if (>= (Variables|攻撃|GetAttack%20Cool%20Down%20Time) 0.0)
            (bind _output_get_2 (Variables|攻撃|SetAttack%20Cool%20Down%20Time (- (Variables|攻撃|GetAttack%20Cool%20Down%20Time) (Variables|Default|GetTime))))
            (Class|BPEnemyAIConInterface|UpdateAttackCoolDownTimeKey(Message) (Variables|Actor|GetAIController) _output_get_2)))
        (:then_1
          (if (>= (Variables|回避|GetAvoidance%20Cool%20Down%20Time) 0.0)
            (bind _output_get_3 (Variables|回避|SetAvoidance%20Cool%20Down%20Time (- (Variables|回避|GetAvoidance%20Cool%20Down%20Time) (Variables|Default|GetTime))))
            (Class|BPEnemyAIConInterface|UpdateAvoidanceCoolDownTimeKey(Message) (Variables|Actor|GetAIController) _output_get_3)))))
    (:then_5
      (if (Variables|回避|GetShadowFlag)
        ;[1 1 1] 残像処理
        (Class|SkeletalMeshComponent|SnapshotPose (Variables|Character|GetMesh) _snapshot) ; 自身のポーズを取る
        (Game|SpawnActorfromClass "/Game/TNK＿Enemy/Enemy/Shadow/BP_ShadowActor.BP_ShadowActor_C" (Transformation|GetActorTransform) "Undefined" 0 _snapshot 0) ; 残像をスポーンさせる
      ))))

(event EventOnEnemyDamageEvent
  (params (In_Other_Actor :type Actor%20Object%20Reference) (Damage_Parameter :type Damage%20Parameter%20Structure))
  ;[1 1 1] ダメージ処理
  (|CallParentFunction In_Other_Actor Damage_Parameter))

(event EventMove
  (params (Location :type Vector :default "0, 0, 0"))
  (bind _aicontroller (Variables|Actor|GetAIController))
  ;[1 1 1] 移動
  (bind _return (CallFunction|IsAlive self))
  (if _return
    (AI|SetFocus _aicontroller (Variables|Actor|GetPlayerCharacter))
    (AI|AIMoveTo (Variables|Actor|GetAIController) Location 0 -1.0 "Enable" "Default" true true)
    (else
      (AI|ClearFocus _aicontroller))))

(event EventEndPlay
  (params (EndPlayReason :type EEndPlayReason%20Enum :default "Destroyed"))
  (|CallParentFunction EndPlayReason))

(event EventEnemyDamageEnable
  ;[1 1 1] 攻撃処理
  ;;[1 0.9658 0] 攻撃判定を呼び出し
  (|CallParentFunction)
  (Variables|攻撃|SetEnemyAttack%20Frag true))

(event EventHitAnimation
  (bind _aicontroller (Variables|Actor|GetAIController))
  ;[1 1 1] ダメージ処理
  (if (not (Variables|攻撃|GetEnemyAttack%20Frag))
    (if (> (Variables|アーマー|GetSuperArmorValue) 0)
      (Variables|アーマー|SetSuperArmorValue (- (Variables|アーマー|GetSuperArmorValue) 1))
      (Variables|アーマー|SetSuperArmorResetTime 8.0)
      (else
        (Animation|PlayAnimMontage "/Game/TNK＿Enemy/Enemy/Animation/AnimationMontage/Corpse/AM_EnemyDamage.AM_EnemyDamage" 1.0 "None")))
    (bind _return (Class|BPEnemyInterface|IsAlive(Message) self))
    (if _return
      (AI|SetFocus _aicontroller (Variables|Actor|GetPlayerCharacter))
      (Variables|Actor|SetPerceivedActor (Variables|Actor|GetPlayerCharacter))
      (Class|BPEnemyAIConInterface|UpdateTagetActorKey(Message) (Variables|Actor|GetAIController) (Variables|Actor|GetPlayerCharacter))
      (else
        (AI|ClearFocus _aicontroller)))))

(event EventDeadAnimation
  (bind _mesh (Variables|Character|GetMesh))
  ;[1 1 1] ダメージ処理
  (Class|SkeletalMeshComponent|SetAllBodiesSimulatePhysics _mesh true)
  (Collision|SetCollisionEnabled _mesh "PhysicsOnly")
  (Collision|SetCollisionEnabled (Variables|Default|GetEnemy_Attack_1) "NoCollision")
  (AI|Logic|StopLogic (Variables|Default|GetBrain%20Component) ""))

(fn ConstructionScript
  (|CallParentFunction))

(fn UpdateWalkSpeed
  (params (NewWalkSpeed :type Float%20%28single-precision%29))
  (Variables|/Script/Engine.CharacterMovementComponent|SetMaxWalkSpeed (Variables|Character|GetCharacterMovement) NewWalkSpeed))

(fn UpdateKey
  (params (PlayerPawn :type Player%20Pawn%20Object%20Reference))
  (bind _aicontroller (Variables|Actor|GetAIController))
  ;[1 1 1] 常にプレイヤーのAttackFragを更新する
  (Class|BPEnemyAIConInterface|UpdatePlayerAttackFlagKey(Message) _aicontroller (Variables|/Game/Player/Blueprint/Player_Pawn.Player_Pawn_C|GetAttack_frag PlayerPawn))
  ;[1 1 1] パリィ成功したフラグを更新する
  (Class|BPEnemyAIConInterface|UpdateParrySuccessFlagKey(Message) _aicontroller (Variables|パリィ|GetParrySuccessFlag))
  ;[1 1 1] 攻撃の確率の値を更新
  (Class|BPEnemyAIConInterface|UpdateAttackRandomKey(Message) _aicontroller (Variables|AI|GetAttackRandam))
  ;[1 1 1] 回避の確率の値を更新
  (Class|BPEnemyAIConInterface|UpdateAvoidanceRandamKey(Message) _aicontroller (Variables|AI|GetAvoidanceRandam)))

(fn ActorDistance
  (params (TagetActor :type Actor%20Object%20Reference))
  (return (Math|Vector|VectorLengthXY (- (Transformation|GetActorLocation) (Transformation|GetActorLocation TagetActor)))))

(fn ForwardMoveto
  (params (Taget :type Actor%20Object%20Reference) (Moving%20distance :type Float%20%28single-precision%29))
  (return (+ (Transformation|GetActorLocation Taget) (* (Math|Vector|GetForwardVector (Variables|Default|GetCapsuleComponent)) Moving%20distance))))

(fn IsAlive
  (return (> (Variables|Default|GetHP) 0.0)))