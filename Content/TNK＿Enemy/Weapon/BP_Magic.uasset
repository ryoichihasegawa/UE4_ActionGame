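; BP_Magic is an enemy weapon actor, apparently a magic attack, that damages the player on contact.
; On BeginPlay it caches the first BP_EnemyCharacter_Bow found in the level via GetActorOfClass, rather than a specific owner, as its damage source.
; When Collision overlaps a component tagged "Body" on a Player_Pawn, it calls OnDamageEvent with that enemy's EnemyDamageValue, then destroys itself.
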(event OnComponentBeginOverlap(Collision)
  (params (OverlappedComponent :type Primitive%20Component%20Object%20Reference) (OtherActor :type Actor%20Object%20Reference) (OtherComp :type Primitive%20Component%20Object%20Reference) (OtherBodyIndex :type Integer) (bFromSweep :type Boolean) (SweepResult :type Hit%20Result%20Structure%20%28by%20ref%29))
  (if (Components|ComponentHasTag OtherComp "Body")
    ;[1 1 1] playerのダメージ処理
    (bind _asplayer_pawn (Utilities|Casting|CastToPlayer_Pawn OtherActor))
    (Default|OnDamageEvent _asplayer_pawn _asplayer_pawn (Utilities|Struct|MakeDamage_Parameter (Variables|/Game/Enemy_base.Enemy_base_C|GetEnemy_Damage%20Value (Variables|Default|GetEnemyBow))))
    (Actor|DestroyActor)))

(event EventBeginPlay
  (bind _returnvalue (Actor|GetActorOfClass "/Game/TNK＿Enemy/Enemy/BP_EnemyCharacter_Bow.BP_EnemyCharacter_Bow_C"))
  (Variables|Default|SetEnemyBow _returnvalue))

(fn ConstructionScript)