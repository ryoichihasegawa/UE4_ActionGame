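; Boss breath-ball effect actor, judging by its name, that damages the player on contact and removes itself.
; BeginPlay caches the player pawn, and the collision box calls its OnDamageEvent with DamageValue when an overlapping component has the "Body" tag.
; The damage call passes the player itself as the other actor.
; A Delay on Tick destroys the actor after five seconds.
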(event OnComponentBeginOverlap(Effect_Boxcollision)
  (params (OverlappedComponent :type Primitive%20Component%20Object%20Reference) (OtherActor :type Actor%20Object%20Reference) (OtherComp :type Primitive%20Component%20Object%20Reference) (OtherBodyIndex :type Integer) (bFromSweep :type Boolean) (SweepResult :type Hit%20Result%20Structure%20%28by%20ref%29))
  (bind _as_player_pawn (Variables|Default|GetAs%20Player%20Pawn))
  (if (Components|ComponentHasTag OtherComp "Body")
    (Default|OnDamageEvent _as_player_pawn _as_player_pawn (Utilities|Struct|MakeDamage_Parameter (Variables|Default|GetDamage%20Value)))))

(event EventBeginPlay
  (bind _asplayer_pawn (Utilities|Casting|CastToPlayer_Pawn (Game|Player|GetPlayerPawn 0)))
  (Variables|Default|SetAs%20Player%20Pawn _asplayer_pawn))

(event Collision|EventActorBeginOverlap
  (params (OtherActor :type Actor%20Object%20Reference)))

(event EventTick
  (params (DeltaSeconds :type Float%20%28single-precision%29))
  (Utilities|FlowControl|Delay 5.0)
  (Actor|DestroyActor))

(fn ConstructionScript)