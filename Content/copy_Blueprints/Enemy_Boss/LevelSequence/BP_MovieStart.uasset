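; BP_MovieStart is a trigger actor that plays the boss appearance cutscene and then spawns the boss.
; When the player pawn overlaps its Box, a DoOnce gate disables input, then creates and plays a Level Sequence player for SQ_Boss_MovieAppeance.
; The sequence's stop event re-enables input and spawns Enemy_Boss with its default controller at a hardcoded transform.
; Camera fade and transform-origin logic are present but unconnected.
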(event OnComponentBeginOverlap(Box)
  (params (OverlappedComponent :type Primitive%20Component%20Object%20Reference) (OtherActor :type Actor%20Object%20Reference) (OtherComp :type Primitive%20Component%20Object%20Reference) (OtherBodyIndex :type Integer) (bFromSweep :type Boolean) (SweepResult :type Hit%20Result%20Structure%20%28by%20ref%29))
  (Utilities|Casting|CastToPlayer_Pawn OtherActor)
  (Utilities|FlowControl|DoOnce false
    (:Completed
      (Input|DisableInput (Game|Player|GetPlayerPawn 0) (Game|GetPlayerController 0))
      (bind _outactor (Sequencer|Player|CreateLevelSequencePlayer "/Game/copy_Blueprints/Enemy_Boss/LevelSequence/SQ_Boss_MovieAppeance.SQ_Boss_MovieAppeance" (Variables|Default|Getbossmovie_sequencer)))
      (bind _output_get (Variables|Default|Setlevel_boss_sequencer _outactor))
      (Utilities|FlowControl|Sequence
        (:then_0
          (Sequencer|Player|Play (Variables|/Script/LevelSequence.LevelSequenceActor|GetSequencePlayer (Variables|Default|Getlevel_boss_sequencer)) :!class /Script/MovieScene.MovieSceneSequencePlayer))
        (:then_1
          (EventDispatchers|BindEventtoOnStop (Variables|/Script/LevelSequence.LevelSequenceActor|GetSequencePlayer (Variables|Default|Getlevel_boss_sequencer)) (delegate Custom|BossAnimetionEnd)))))))

(event Custom|BossAnimetionEnd
  (Input|EnableInput (Game|Player|GetPlayerPawn 0) (Game|GetPlayerController 0))
  (bind _returnvalue (Game|SpawnActorfromClass "/Game/copy_Blueprints/Enemy_Boss/BP/Enemy_Boss.Enemy_Boss_C" (Math|Transform|MakeTransform "-32980.000000,6260.000000,-900.000000" "0,0.000000,0.000000" "1.500000,1.500000,1.500000") "AlwaysSpawn" 0 0))
  (Pawn|SpawnDefaultController _returnvalue))

(event EventBeginPlay)

(event Collision|EventActorBeginOverlap
  (params (OtherActor :type Actor%20Object%20Reference)))

(event EventTick
  (params (DeltaSeconds :type Float%20%28single-precision%29)))

(fn ConstructionScript)