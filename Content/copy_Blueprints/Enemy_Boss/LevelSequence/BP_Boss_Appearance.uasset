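; Trigger actor that plays the boss appearance cutscene when the player pawn enters its Box.
; On overlap it disables player input, creates a player for SQ_Boss_Appearance and starts it, re-enabling input through a callback bound to the sequence's stop.
; The sequence's instance data is overridden so its transform origin is the player pawn, placing the cutscene relative to the player.
; The overlap has no one-shot guard.
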(event OnComponentBeginOverlap(Box)
  (params (OverlappedComponent :type Primitive%20Component%20Object%20Reference) (OtherActor :type Actor%20Object%20Reference) (OtherComp :type Primitive%20Component%20Object%20Reference) (OtherBodyIndex :type Integer) (bFromSweep :type Boolean) (SweepResult :type Hit%20Result%20Structure%20%28by%20ref%29))
  (bind _returnvalue (Game|Player|GetPlayerPawn 0))
  (Utilities|Casting|CastToPlayer_Pawn OtherActor)
  (Input|DisableInput (Game|GetPlayerController 0))
  (bind _outactor (Sequencer|Player|CreateLevelSequencePlayer "/Game/copy_Blueprints/Enemy_Boss/LevelSequence/SQ_Boss_Appearance.SQ_Boss_Appearance"))
  (bind _output_get (Variables|Default|SetOut%20Actor _outactor))
  (Variables|/Script/LevelSequence.LevelSequenceActor|SetbOverrideInstanceData _output_get true)
  (Utilities|FlowControl|Sequence
    (:then_0
      (Variables|/Script/LevelSequence.DefaultLevelSequenceInstanceData|SetTransformOriginActor (.AsDefault%20Level%20Sequence%20Instance%20Data (Utilities|Casting|CastToDefaultLevelSequenceInstanceData (Variables|/Script/LevelSequence.LevelSequenceActor|GetDefaultInstanceData (Variables|Default|GetOut%20Actor)))) _returnvalue)
      (Variables|/Script/LevelSequence.DefaultLevelSequenceInstanceData|SetTransformOrigin (.AsDefault%20Level%20Sequence%20Instance%20Data (Utilities|Casting|CastToDefaultLevelSequenceInstanceData (Variables|/Script/LevelSequence.LevelSequenceActor|GetDefaultInstanceData (Variables|Default|GetOut%20Actor)))) (Transformation|GetActorTransform _returnvalue)))
    (:then_1
      (EventDispatchers|BindEventtoOnStop (Variables|/Script/LevelSequence.LevelSequenceActor|GetSequencePlayer (Variables|Default|GetOut%20Actor)) (delegate Custom|finishAnimation)))
    (:then_2
      (Sequencer|Player|Play (Variables|/Script/LevelSequence.LevelSequenceActor|GetSequencePlayer (Variables|Default|GetOut%20Actor)) :!class /Script/MovieScene.MovieSceneSequencePlayer))))

(event Custom|finishAnimation
  (Input|EnableInput (Game|GetPlayerController 0)))

(event EventBeginPlay)

(event Collision|EventActorBeginOverlap
  (params (OtherActor :type Actor%20Object%20Reference)))

(event EventTick
  (params (DeltaSeconds :type Float%20%28single-precision%29)))

(fn ConstructionScript)