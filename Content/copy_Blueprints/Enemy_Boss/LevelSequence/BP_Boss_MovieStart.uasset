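; Boss-intro trigger actor that plays the boss appearance cinematic and starts battle music.
; The first player overlap plays the Level Sequence with input and HUD disabled; when it stops, both return, a boss spawn-reset dispatcher fires and BGM starts.
; Tick watches player HP; at zero it re-arms a second trigger, whose next overlap restarts boss AI and music through dispatchers and a spawned 2D sound.
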(event OnComponentBeginOverlap(play_bossMovie)
  (params (OverlappedComponent :type Primitive%20Component%20Object%20Reference) (OtherActor :type Actor%20Object%20Reference) (OtherComp :type Primitive%20Component%20Object%20Reference) (OtherBodyIndex :type Integer) (bFromSweep :type Boolean) (SweepResult :type Hit%20Result%20Structure%20%28by%20ref%29))
  (Utilities|Casting|CastToPlayer_Pawn OtherActor)
  (Utilities|FlowControl|DoOnce false
    (:Completed
      (Collision|SetCollisionEnabled (Variables|Default|Getplay_bossMovie) "NoCollision")
      (Input|DisableInput (Game|Player|GetPlayerPawn 0) (Game|GetPlayerController 0))
      (bind _outactor (Sequencer|Player|CreateLevelSequencePlayer "/Game/copy_Blueprints/Enemy_Boss/LevelSequence/SQ_Boss_MovieAppeance.SQ_Boss_MovieAppeance" (Variables|Default|Getbossmovie_sequencer)))
      (bind _output_get (Variables|Default|Setlevel_boss_sequencer _outactor))
      (Utilities|FlowControl|Sequence
        (:then_0
          (Sequencer|Player|Play (Variables|/Script/LevelSequence.LevelSequenceActor|GetSequencePlayer (Variables|Default|Getlevel_boss_sequencer)) :!class /Script/MovieScene.MovieSceneSequencePlayer)
          (Default|DeleteWidget (Variables|Default|GetAs%20Player%20Pawn)))
        (:then_1
          (EventDispatchers|BindEventtoOnStop (Variables|/Script/LevelSequence.LevelSequenceActor|GetSequencePlayer (Variables|Default|Getlevel_boss_sequencer)) (delegate Custom|BossAnimetionEnd)))))))

(event OnComponentBeginOverlap(play_againBGM)
  (params (OverlappedComponent :type Primitive%20Component%20Object%20Reference) (OtherActor :type Actor%20Object%20Reference) (OtherComp :type Primitive%20Component%20Object%20Reference) (OtherBodyIndex :type Integer) (bFromSweep :type Boolean) (SweepResult :type Hit%20Result%20Structure%20%28by%20ref%29))
  (Utilities|Casting|CastToPlayer_Pawn OtherActor)
  (Utilities|FlowControl|DoOnce false
    (:Completed
      (Default|CallBossRestartAI)
      (Collision|SetCollisionEnabled (Variables|Default|Getplay_againBGM) "NoCollision")
      (CallFunction|PlayBossBGM)
      (Default|CallBossRestartAI))))

(event Custom|BossAnimetionEnd
  (Variables|Default|Setplayer_setPosition true)
  (Default|CallBossRssetspawn)
  (Input|EnableInput (Game|Player|GetPlayerPawn 0) (Game|GetPlayerController 0))
  (Default|CreateWidget (Variables|Default|GetAs%20Player%20Pawn))
  (CallFunction|PlayBossBGM))

(event Custom|Rsset_BossBGM
  (Utilities|FlowControl|DoOnce false) ; enters at Reset
)

(event EventBeginPlay
  (Collision|SetCollisionEnabled (Variables|Default|Getplay_againBGM) "NoCollision")
  (bind _asplayer_pawn (Utilities|Casting|CastToPlayer_Pawn (Game|Player|GetPlayerPawn 0)))
  (Utilities|IsValid _asplayer_pawn
    (:Is%20Valid
      (Variables|Default|SetAs%20Player%20Pawn _asplayer_pawn))))

(event Collision|EventActorBeginOverlap
  (params (OtherActor :type Actor%20Object%20Reference)))

(event EventTick
  (params (DeltaSeconds :type Float%20%28single-precision%29))
  (Utilities|FlowControl|Sequence
    (:then_0
      (if (<= (.Value (Utilities|Map|Find (Variables|/Game/Player/Blueprint/Player_Pawn.Player_Pawn_C|GetStatus (Variables|Default|GetAs%20Player%20Pawn)) "HP")) 0.0)
        (Collision|SetCollisionEnabled (Variables|Default|Getplay_againBGM) "QueryAndPhysics")
        (CallFunction|RssetBossBGM)))))

(fn ConstructionScript)

(fn PlayBossBGM
  (bind _returnvalue (Audio|SpawnSound2D (Variables|Default|Getm_battlesound) 1.0 1.0 0.0 0))
  (bind _output_get (Variables|Default|Setboss_battleSound _returnvalue))
  (Default|CallBossBattleSoundEvent _output_get))

(fn BossAttack
  (return 0.0))