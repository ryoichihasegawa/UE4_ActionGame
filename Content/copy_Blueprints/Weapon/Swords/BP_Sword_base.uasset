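; Base sword weapon Blueprint that attaches its mesh to a socket on the player character's skeletal mesh.
; On BeginPlay it enables input from the first player controller and caches the BP_Player_001 reference.
; SetAttachment stores the given hand socket name and attaches the PlayerMesh component there with relative transform rules.
; The sub-socket attachment branch is disconnected, so that parameter has no effect.
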(event EventBeginPlay
  ;[1 1 1] キー入力イベントを受け入れるようにする
  (Input|EnableInput (Game|GetPlayerController 0))
  (bind _asbp_player_001 (Utilities|Casting|CastToBP_Player_001 (Game|GetPlayerCharacter 0)))
  (Variables|Default|SetPlayer _asbp_player_001))

(fn ConstructionScript)

(fn SetAttachment
  (params (SetHandSocket :type Name) (SetSubSocket :type Name))
  (bind _output_get (Variables|Default|SetSocketHandName SetHandSocket))
  (Transformation|AttachComponentToComponent (Variables|Default|GetPlayerMesh) (Variables|/Script/Engine.Character|GetMesh (.AsBP%20Player%20001 (Utilities|Casting|CastToBP_Player_001 (Game|GetPlayerCharacter 0)))) _output_get "KeepRelative" "KeepRelative" "KeepRelative" true))