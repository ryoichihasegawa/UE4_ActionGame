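; Player shield Blueprint that attaches to the shield socket and detects frontal blocks of enemy attacks.
; ShieldCollision overlaps count only while the player's State is guard and the component is tagged Enemy_Attack.
; ShieldRange accepts an Enemy_Boss within 90 degrees of player forward via dot product, triggering a Niagara impact at the player, with debug prints.
; EnableCollision and DisableCollision events toggle the guard collision, intended for use during animations.
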(event OnComponentBeginOverlap(ShieldCollision)
  (params (OverlappedComponent :type Primitive%20Component%20Object%20Reference) (OtherActor :type Actor%20Object%20Reference) (OtherComp :type Primitive%20Component%20Object%20Reference) (OtherBodyIndex :type Integer) (bFromSweep :type Boolean) (SweepResult :type Hit%20Result%20Structure%20%28by%20ref%29))
  ;[1 1 1] ガードコリジョン
  ;;[1 0.276 0.276] PlayerのStateがガードになっているか
  (if (Utilities|Enum|Equal(Enum) (Variables|/Game/copy_Blueprints/Character/Character/Player_001/BP_Player_001.BP_Player_001_C|GetState (Variables|Default|GetPlayer)) "NewEnumerator2")
    ;;[1 0.2604 0.2604] Enemy_Attackタグに当たったか
    (if (Components|ComponentHasTag OtherComp "Enemy_Attack")
      ;;[1 1 1] Enemyの攻撃ベクトルがシールドの回転ベクトル範囲以内か
      (if (CallFunction|ShieldRange OtherActor)
        (Default|OnCollisionEvent self (Variables|Default|GetPlayer))
        (Development|PrintString "前から")
        (else
          (Development|PrintString "後ろから"))))))

(event EventBeginPlay
  (CallFunction|SetAttachment "shield_ソケット") ; ゲームが始まった時にシールドを持たせる
  (bind _asbp_player_001 (Utilities|Casting|CastToBP_Player_001 (Game|GetPlayerCharacter 0)))
  (Variables|Default|SetPlayer _asbp_player_001))

(event Collision|EventActorBeginOverlap
  (params (OtherActor :type Actor%20Object%20Reference))
  (|CallParentFunction OtherActor) ; このノードは無効になっているため呼び出せません。\n機能をビルドするにはピンをドラッグしてください。
)

(event EventTick
  (params (DeltaSeconds :type Float%20%28single-precision%29))
  (|CallParentFunction DeltaSeconds) ; このノードは無効になっているため呼び出せません。\n機能をビルドするにはピンをドラッグしてください。
)

(event EventDisableCollision
  ;[1 1 1] アニメーション中ガードコリジョン
  (Collision|SetCollisionEnabled (Variables|Default|GetShieldCollision) "NoCollision"))

(event EventEnableCollision
  ;[1 1 1] アニメーション中ガードコリジョン
  (Collision|SetCollisionEnabled (Variables|Default|GetShieldCollision) "QueryAndPhysics"))

(event EventOnCollisionEvent
  (params (inPlayer :type Actor%20Object%20Reference))
  (Niagara|SpawnSystematLocation "/Game/Hack_And_Slash_FX/VFX_Niagara/Impacts/NS_Lightning_Slash_Impact.NS_Lightning_Slash_Impact" (Transformation|GetActorLocation inPlayer)))

(fn ConstructionScript
  (|CallParentFunction))

(fn ShieldRange
  (params (OtherActor :type Actor%20Object%20Reference))
  (bind _asenemy_boss (Utilities|Casting|CastToEnemy_Boss OtherActor))
  (bind _player (Variables|Default|GetPlayer))
  (bind _returnvalue (Transformation|GetActorLocation _asenemy_boss))
  (bind _returnvalue_2 (Transformation|GetActorForwardVector _player))
  (bind _returnvalue_3 (Transformation|GetActorLocation _player))
  (bind _returnvalue_4 (Math|Rotator|FindLookatRotation _returnvalue_3 _returnvalue))
  (bind _returnvalue_5 (Math|Vector|GetForwardVector _returnvalue_4))
  (bind _returnvalue_6 (Math|Vector|DotProduct _returnvalue_2 _returnvalue_5))
  (bind _returnvalue_7 (Class|KismetMathLibrary|DegAcos _returnvalue_6))
  (Development|PrintString (Utilities|String|ToString(Float) _returnvalue_7))
  (Development|PrintString (Utilities|String|ToString(Float) (Class|KismetMathLibrary|DegAcos (Math|Vector|DotProduct (Math|Vector|GetForwardVector (Variables|/Script/Engine.Actor|GetRootComponent _player)) (Math|Vector|GetForwardVector (Math|Rotator|FindLookatRotation (Transformation|GetWorldLocation (Variables|Default|GetStandardArrow)) (Transformation|GetWorldLocation (Variables|Default|GetPibotArrow))))))))
  (return (< _returnvalue_7 9e+01)))