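; Base weapon actor that the player picks up on overlap and can later throw.
; On overlap with a Player-tagged Player_Pawn, it disables box collision, joins WeponList, attaches to the Sword_Main_Socket and ends up hidden.
; PickUpFrag, HaveFrag and ThrowFrag gate collision, visibility and throwing.
; Throwing moves the box to ThrowPosition and reshows the mesh without detaching; Tick and ThrowWeponLocation are stubs.
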(event OnComponentBeginOverlap(e)
  (params (OverlappedComponent :type Primitive%20Component%20Object%20Reference) (OtherActor :type Actor%20Object%20Reference) (OtherComp :type Primitive%20Component%20Object%20Reference) (OtherBodyIndex :type Integer) (bFromSweep :type Boolean) (SweepResult :type Hit%20Result%20Structure%20%28by%20ref%29))
  ;[1 1 1] 拾われるとき
  (if (not (Variables|Default|GetPickUp_Frag))
    (if (Actor|ActorHasTag OtherActor "Player")
      (CallFunction|CollsionSet)
      (bind _asplayer_pawn (Utilities|Casting|CastToPlayer_Pawn OtherActor))
      (bind _returnvalue (Utilities|Array|Add (Variables|/Game/Player/Blueprint/Player_Pawn.Player_Pawn_C|GetWepon_List _asplayer_pawn) self))
      (Development|PrintString (Utilities|String|ToString(Integer) _returnvalue))
      (if (== _returnvalue 1)
        (Variables|Default|SetHave_Frag true)
        (CallFunction|VisibillityWepon))
      (Transformation|AttachComponentToComponent (Variables|/Script/Engine.Character|GetMesh _asplayer_pawn) "Sword_Main_Socket" "SnapToTarget" "SnapToTarget" "SnapToTarget" true)
      (Variables|Default|SetPickUp_Frag true)
      (Variables|Default|SetHave_Frag false)
      (CallFunction|VisibillityWepon))))

(event Custom|Visibillity_Wepon
  (bind _skeletalmesh (Variables|Default|GetSkeletalMesh))
  (if (Variables|Default|GetPickUp_Frag)
    (if (Variables|Default|GetHave_Frag)
      (Rendering|SetVisibility _skeletalmesh true false)
      (else
        (Rendering|SetVisibility _skeletalmesh false false)))))

(event Custom|Collsion_Set
  (bind _box (Variables|Default|GetBox))
  (if (Variables|Default|GetPickUp_Frag)
    (Collision|SetCollisionEnabled _box "QueryAndPhysics")
    (else
      (Collision|SetCollisionEnabled _box "NoCollision"))))

(event Custom|Wepon_Throw
  (if (Variables|Default|GetThrow_Frag)
    (Transformation|SetWorldLocation (Variables|Default|GetBox) (Variables|Default|GetThrow_Position) false false)
    (Variables|Default|SetPickUp_Frag false)
    (Variables|Default|SetHave_Frag false)
    (Variables|Default|SetThrow_Frag false)
    (Rendering|SetVisibility (Variables|Default|GetSkeletalMesh) true false)))

(event EventBeginPlay)

(event Collision|EventActorBeginOverlap
  (params (OtherActor :type Actor%20Object%20Reference)))

(event EventTick
  (params (DeltaSeconds :type Float%20%28single-precision%29))
  (Utilities|FlowControl|Sequence))

(fn ConstructionScript)

(fn ThrowWeponLocation
  (params (Location :type Vector :default "0, 0, 0"))
  (return "0, 0, 0"))