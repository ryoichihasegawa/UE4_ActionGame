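; Test actor, apparently for experimenting with guard direction math between itself and the player.
; Only BeginPlay does work, caching the Player_Pawn; the Box overlap checks a "Player" tag but takes no action, and Tick and hit are empty.
; Disconnected debug chains print arrow vectors and orient and scale indicator arrows from summed player and local directions.
; An unused calculation derives the angle between the player's Gard facing and this actor.
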(event OnComponentBeginOverlap(Box)
  (params (OverlappedComponent :type Primitive%20Component%20Object%20Reference) (OtherActor :type Actor%20Object%20Reference) (OtherComp :type Primitive%20Component%20Object%20Reference) (OtherBodyIndex :type Integer) (bFromSweep :type Boolean) (SweepResult :type Hit%20Result%20Structure%20%28by%20ref%29))
  (if (Actor|ActorHasTag OtherActor "Player")
    _))

(event OnComponentHit(Box)
  (params (HitComponent :type Primitive%20Component%20Object%20Reference) (OtherActor :type Actor%20Object%20Reference) (OtherComp :type Primitive%20Component%20Object%20Reference) (NormalImpulse :type Vector :default "0, 0, 0") (Hit :type Hit%20Result%20Structure%20%28by%20ref%29)))

(event EventBeginPlay
  (bind _asplayer_pawn (Utilities|Casting|CastToPlayer_Pawn (Game|Player|GetPlayerPawn 0)))
  (Variables|Default|SetPlayer _asplayer_pawn))

(event EventTick
  (params (DeltaSeconds :type Float%20%28single-precision%29)))

(fn ConstructionScript)