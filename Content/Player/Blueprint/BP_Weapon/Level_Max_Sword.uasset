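; Max-level sword weapon Blueprint for the player, the Dragon Slayer Sword (竜殺しの剣).
; BeginPlay runs the parent's logic, then fills in weapon variables for name, description, texture, mesh, attack and speed.
; It is a data-only variant in practice: the construction script just calls the parent, and the overlap and Tick events are inactive.
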(event EventBeginPlay
  (|CallParentFunction)
  (Variables|Default|SetWepon_Name "竜殺しの剣")
  (Variables|Default|SetWepon_Explain "ATK  50")
  (Variables|Default|SetWepon_Texture "/Game/Player/UI/Texture/Sword_level_max2.Sword_level_max2")
  (Variables|Default|SetWepon＿Me "/Game/Player/Weapon/Swords/Blade_DragonSword/SK_Blade_DragonSword.SK_Blade_DragonSword")
  (Variables|Default|SetWepon_ATK 5e+01)
  (Variables|Default|SetWepon_speed 1.2))

(event Collision|EventActorBeginOverlap
  (params (OtherActor :type Actor%20Object%20Reference)))

(event EventTick
  (params (DeltaSeconds :type Float%20%28single-precision%29))
  (|CallParentFunction DeltaSeconds) ; このノードは無効になっているため呼び出せません。\n機能をビルドするにはピンをドラッグしてください。
)

(fn ConstructionScript
  (|CallParentFunction))