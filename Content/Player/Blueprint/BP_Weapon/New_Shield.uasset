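; Player's shield weapon, which attaches to the shield socket on BeginPlay and provides directional guarding.
; On shield collision overlap while the player is guarding, ShieldRange uses a forward-vector dot product to confirm the other actor is in front, then sets the player's DamageCut.
; Events toggle the guard collision and spawn a lightning impact effect at a given actor.
; Tick hides the mesh while the player is dead.
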(event OnComponentBeginOverlap(ShieldCollision)
  (params (OverlappedComponent :type Primitive%20Component%20Object%20Reference) (OtherActor :type Actor%20Object%20Reference) (OtherComp :type Primitive%20Component%20Object%20Reference) (OtherBodyIndex :type Integer) (bFromSweep :type Boolean) (SweepResult :type Hit%20Result%20Structure%20%28by%20ref%29))
  ;[1 1 1] ガードコリジョン
  ;;[1 0.276 0.276] PlayerのStateがガードになっているか
  (if (Variables|/Game/Player/Blueprint/Player_Pawn.Player_Pawn_C|GetGard_frag (Variables|Default|GetPlayer))
    ;;[1 1 1] Enemyの攻撃ベクトルがシールドの回転ベクトル範囲以内か
    (if (CallFunction|ShieldRange OtherActor)
      (Variables|/Game/Player/Blueprint/Player_Pawn.Player_Pawn_C|SetDamage_Cut (Variables|Default|GetPlayer) 5.0))))

(event EventBeginPlay
  (CallFunction|SetAttachment "shield_ソケット") ; ゲームが始まった時にシールドを持たせる
  (bind _asplayer_pawn (Utilities|Casting|CastToPlayer_Pawn (Game|GetPlayerCharacter 0)))
  (Variables|Default|SetPlayer _asplayer_pawn))

(event Collision|EventActorBeginOverlap
  (params (OtherActor :type Actor%20Object%20Reference))
  (|CallParentFunction OtherActor) ; このノードは無効になっているため呼び出せません。\n機能をビルドするにはピンをドラッグしてください。
)

(event EventTick
  (params (DeltaSeconds :type Float%20%28single-precision%29))
  (if (Variables|/Game/Player/Blueprint/Player_Pawn.Player_Pawn_C|GetIsDead (Variables|Default|GetPlayer))
    (Rendering|SetVisibility (Variables|Default|GetShieldMesh) false false)
    (else
      (Rendering|SetVisibility (Variables|Default|GetShieldMesh) true false))))

(event EventDisableCollision
  ;[1 1 1] アニメーション中ガードコリジョン
  (Collision|SetCollisionEnabled (Variables|Default|GetShieldCollision) "NoCollision"))

(event EventEnableCollision
  ;[1 1 1] アニメーション中ガードコリジョン
  (Collision|SetCollisionEnabled (Variables|Default|GetShieldCollision) "QueryAndPhysics"))

(event EventOnCollisionEvent
  (params (inPlayer :type Actor%20Object%20Reference))
  (Niagara|SpawnSystematLocation "/Game/Hack_And_Slash_FX/VFX_Niagara/Impacts/NS_Lightning_Slash_Impact.NS_Lightning_Slash_Impact" (Transformation|GetActorLocation inPlayer)))

(fn ConstructionScript
  (|CallParentFunction))

(fn ShieldRange
  (params (OtherActor :type Actor%20Object%20Reference))
  (bind _returnvalue (Transformation|GetActorLocation OtherActor))
  (bind _player (Variables|Default|GetPlayer))
  (bind _returnvalue_2 (Transformation|GetActorLocation _player))
  (bind _returnvalue_3 (Math|Rotator|FindLookatRotation _returnvalue_2 _returnvalue))
  (Transformation|SetWorldRotation (Variables|Default|GetStandardArrow) _returnvalue_3 false false)
  (return (< (Class|KismetMathLibrary|DegAcos (Math|Vector|DotProduct (Math|Vector|GetForwardVector (Variables|/Game/Player/Blueprint/Character_base.Character_base_C|GetCharacter_Forward_vector _player)) (Math|Vector|GetForwardVector _returnvalue_3))) 9e+01)))