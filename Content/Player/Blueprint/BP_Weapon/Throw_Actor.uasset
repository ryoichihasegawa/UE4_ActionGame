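; Thrown weapon actor that takes the player's throw-weapon mesh on spawn and resolves what it hits.
; On box overlap with an Enemy or Map tag it records the hit location on Player_Pawn.
; Only if the Enemy_base cast succeeds does it deal PlayerATK damage, call WeponGroundHit, create weapon UI and destroy itself.
; Sword_Change hits record location, call WeponGroundHit and destroy the actor without damage.
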(event OnComponentBeginOverlap(Box)
  (params (OverlappedComponent :type Primitive%20Component%20Object%20Reference) (OtherActor :type Actor%20Object%20Reference) (OtherComp :type Primitive%20Component%20Object%20Reference) (OtherBodyIndex :type Integer) (bFromSweep :type Boolean) (SweepResult :type Hit%20Result%20Structure%20%28by%20ref%29))
  ;[1 1 1] 敵やオブジェクトに当たった時の処理
  (if (or (Actor|ActorHasTag OtherActor "Enemy") (Actor|ActorHasTag OtherActor "Map"))
    (bind _asplayer_pawn (Utilities|Casting|CastToPlayer_Pawn (Game|Player|GetPlayerPawn 0)))
    (Variables|/Game/Player/Blueprint/Player_Pawn.Player_Pawn_C|Setwepon_throw_location%20 _asplayer_pawn (Transformation|GetActorLocation))
    (bind _asenemy_base (Utilities|Casting|CastToEnemy_base OtherActor))
    (Default|OnEnemyDamageEvent _asenemy_base OtherActor (Utilities|Struct|MakeDamage_Parameter (Variables|/Game/Player/Blueprint/Character_base.Character_base_C|GetPlayer_ATK _asplayer_pawn)))
    (Default|WeponGroundHit _asplayer_pawn)
    (Default|WeponUICreate (Variables|/Game/Player/Blueprint/Player_Pawn.Player_Pawn_C|GetAction_game_UI _asplayer_pawn))
    (Actor|DestroyActor)
    (elif (Actor|ActorHasTag OtherActor "Sword_Change")
      (bind _asplayer_pawn_2 (Utilities|Casting|CastToPlayer_Pawn (Game|Player|GetPlayerPawn 0)))
      (Variables|/Game/Player/Blueprint/Player_Pawn.Player_Pawn_C|Setwepon_throw_location%20 _asplayer_pawn_2 (Transformation|GetActorLocation))
      (Default|WeponGroundHit _asplayer_pawn_2)
      (Actor|DestroyActor))))

(event EventBeginPlay
  (bind _asplayer_pawn (Utilities|Casting|CastToPlayer_Pawn (Game|Player|GetPlayerPawn 0)))
  (Class|SkinnedMeshComponent|SetSkeletalMesh (Variables|Default|GetSkeletalMesh) (Variables|/Game/Player/Blueprint/Player_Pawn.Player_Pawn_C|GetThrow_Wepon _asplayer_pawn) false))

(event Collision|EventActorBeginOverlap
  (params (OtherActor :type Actor%20Object%20Reference)))

(fn ConstructionScript)