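; Base weapon actor that the player can pick up, carry and throw.
; Overlapping the pickup collision opens a gate that Tick polls until the player's Pickup flag is set, then the weapon joins WeponList and attaches to Sword_Main_Socket.
; Only the held weapon, initially the first collected, is visible and copies its attack and speed to Player_Pawn.
; Throwing moves its Box to ThrowPosition, clears the carry flags and shows the mesh.
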(event OnComponentBeginOverlap(PickUp＿Collsion)
  (params (OverlappedComponent :type Primitive%20Component%20Object%20Reference) (OtherActor :type Actor%20Object%20Reference) (OtherComp :type Primitive%20Component%20Object%20Reference) (OtherBodyIndex :type Integer) (bFromSweep :type Boolean) (SweepResult :type Hit%20Result%20Structure%20%28by%20ref%29))
  ;[1 1 1] 拾われるとき
  (if (not (Variables|フラグ|GetPickUp_Frag))
    (if (Actor|ActorHasTag OtherActor "Player")
      (Variables|フラグ|SetPickUpGate_Frag true)
      (bind _asplayer_pawn (Utilities|Casting|CastToPlayer_Pawn OtherActor))
      (Variables|/Game/Player/Blueprint/Player_Pawn.Player_Pawn_C|SetPick_Up_frag _asplayer_pawn true))))

(event OnComponentEndOverlap(PickUp＿Collsion)
  (params (OverlappedComponent :type Primitive%20Component%20Object%20Reference) (OtherActor :type Actor%20Object%20Reference) (OtherComp :type Primitive%20Component%20Object%20Reference) (OtherBodyIndex :type Integer))
  ;[1 1 1] 取られなかったとき
  (if (Variables|フラグ|GetPickUp_Frag)
    (Variables|フラグ|SetPickUpGate_Frag false)
    (elif (Actor|ActorHasTag OtherActor "Player")
      (Variables|フラグ|SetPickUpGate_Frag false))))

(event Custom|Visibillity_Wepon
  (bind _skeletalmesh (Variables|Default|GetSkeletalMesh))
  ;[1 1 1] 武器の透明化の処理
  (if (Variables|フラグ|GetPickUp_Frag)
    (if (Variables|フラグ|GetHave_Frag)
      (Rendering|SetVisibility _skeletalmesh true false)
      (bind _asplayer_pawn (Utilities|Casting|CastToPlayer_Pawn (Game|Player|GetPlayerPawn 0)))
      (Variables|/Game/Player/Blueprint/Character_base.Character_base_C|SetPlayer_ATK _asplayer_pawn (Variables|武器ステ|GetWepon_ATK))
      (Variables|/Game/Player/Blueprint/Player_Pawn.Player_Pawn_C|SetAttack_Speed _asplayer_pawn (Variables|武器ステ|GetWepon_speed))
      (else
        (Rendering|SetVisibility _skeletalmesh false false)))))

(event Custom|Pick_Start
  ;[1 1 1] 拾う状態
  (bind _asplayer_pawn (Utilities|Casting|CastToPlayer_Pawn (Game|Player|GetPlayerPawn 0)))
  (if (Variables|/Game/Player/Blueprint/Player_Pawn.Player_Pawn_C|GetPickup _asplayer_pawn)
    (Variables|フラグ|SetPickUp_Frag true)
    (CallFunction|CollsionSet)
    (Variables|/Game/Player/Blueprint/Player_Pawn.Player_Pawn_C|SetWeapon_frag _asplayer_pawn true)
    (bind _returnvalue (Utilities|Array|Add (Variables|/Game/Player/Blueprint/Player_Pawn.Player_Pawn_C|GetWepon_List _asplayer_pawn) self))
    (Transformation|AttachComponentToComponent (Variables|/Script/Engine.Character|GetMesh _asplayer_pawn) "Sword_Main_Socket" "SnapToTarget" "SnapToTarget" "SnapToTarget" true)
    (Variables|フラグ|SetPickUpGate_Frag false)
    (if (== _returnvalue 0)
      (Variables|フラグ|SetHave_Frag true)
      (CallFunction|VisibillityWepon)
      (else
        (Variables|フラグ|SetHave_Frag false)
        (CallFunction|VisibillityWepon)))))

(event Custom|Collsion_Set
  (bind _box (Variables|Default|GetBox))
  ;[1 1 1] 拾う用の判定のＯＮ/ＯＦＦ
  (if (Variables|フラグ|GetPickUp_Frag)
    (Collision|SetCollisionEnabled _box "NoCollision")
    (else
      (Collision|SetCollisionEnabled _box "QueryAndPhysics"))))

(event Custom|Wepon_Throw
  ;[1 1 1] 投げる処理
  (if (Variables|投げる関連|GetThrow_Frag)
    (Transformation|SetWorldLocation (Variables|Default|GetBox) (Variables|投げる関連|GetThrow_Position) false false)
    (Variables|フラグ|SetPickUp_Frag false)
    (Variables|フラグ|SetHave_Frag false)
    (Variables|投げる関連|SetThrow_Frag false)
    (Rendering|SetVisibility (Variables|Default|GetSkeletalMesh) true false)))

(event EventTick
  (params (DeltaSeconds :type Float%20%28single-precision%29))
  (if (Variables|フラグ|GetPickUpGate_Frag)
    (CallFunction|PickStart)))

(event EventPickUpCollsionDisabled
  ;[1 1 1] 拾う用の判定のＯＮ/ＯＦＦ
  (Collision|SetCollisionEnabled (Variables|Default|GetPickUp＿Collsion) "NoCollision"))

(event EventPickUpCollsionEnabled
  ;[1 1 1] 拾う用の判定のＯＮ/ＯＦＦ
  (Collision|SetCollisionEnabled (Variables|Default|GetPickUp＿Collsion) "QueryAndPhysics"))

(event EventBeginPlay
  ;[1 1 1] 初期化
  (Class|SkinnedMeshComponent|SetSkeletalMesh (Variables|Default|GetSkeletalMesh) (Variables|投げる関連|GetWepon＿Me) true))

(fn ConstructionScript)

(fn ThrowWeponLocation
  (params (Location :type Vector :default "0, 0, 0"))
  (return "0, 0, 0"))