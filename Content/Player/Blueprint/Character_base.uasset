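; Player character base Blueprint that handles melee-style attack hits against enemies.
; An attack collision overlap with an Enemy-tagged Enemy_base triggers hit stop and camera shake, then sends player attack damage through its damage event.
; Two events toggle the attack collision on and off.
; The Hit_Stop macro briefly slows global time dilation, then restores normal speed after a delay.
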(event OnComponentBeginOverlap(Player_Attack_Collsion)
  (params (OverlappedComponent :type Primitive%20Component%20Object%20Reference) (OtherActor :type Actor%20Object%20Reference) (OtherComp :type Primitive%20Component%20Object%20Reference) (OtherBodyIndex :type Integer) (bFromSweep :type Boolean) (SweepResult :type Hit%20Result%20Structure%20%28by%20ref%29))
  ;[1 1 1] 判定
  (if (or (Actor|ActorHasTag OtherActor "Enemy") (Actor|ActorHasTag OtherActor "Enemy1"))
    (bind _asenemy_base (Utilities|Casting|CastToEnemy_base OtherActor))
    (Utilities|HitStop 0.1 0.02)
    (Game|Feedback|ClientStartCameraShake (Game|GetPlayerController 0) "/Game/Player/Blueprint/Camera_Shake_2.Camera_Shake_2_C" 1.0 "CameraLocal" "0, 0, 0")
    (Default|OnEnemyDamageEvent _asenemy_base OtherActor (Utilities|Struct|MakeDamage_Parameter (Variables|Default|GetPlayer_ATK)))))

(event Collision|EventActorBeginOverlap
  (params (OtherActor :type Actor%20Object%20Reference)))

(event EventDamageCollsionDisabled
  ;[1 1 1] Front_Collsion
  (Collision|SetCollisionEnabled (Variables|Default|GetPlayer_Attack_Collsion) "NoCollision"))

(event EventDamageCollsionEnabled
  ;[1 1 1] Front_Collsion
  (Collision|SetCollisionEnabled (Variables|Default|GetPlayer_Attack_Collsion) "QueryAndPhysics"))

(fn ConstructionScript)