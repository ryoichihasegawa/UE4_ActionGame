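; Sword pickup actor that the player collects by touching it, joining their weapon list.
; When component E begins an overlap with an actor tagged Player, it casts to Player_Pawn, adds itself to WeponList and snap-attaches to the wepon_2 socket on the pawn's mesh.
; The PickUpFrag flag then blocks any further pickup.
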(event OnComponentBeginOverlap(e)
  (params (OverlappedComponent :type Primitive%20Component%20Object%20Reference) (OtherActor :type Actor%20Object%20Reference) (OtherComp :type Primitive%20Component%20Object%20Reference) (OtherBodyIndex :type Integer) (bFromSweep :type Boolean) (SweepResult :type Hit%20Result%20Structure%20%28by%20ref%29))
  (if (not (Variables|Default|GetPickUp_frag))
    (if (Actor|ActorHasTag OtherActor "Player")
      (bind _asplayer_pawn (Utilities|Casting|CastToPlayer_Pawn OtherActor))
      (Utilities|Array|Add (Variables|/Game/Player/Blueprint/Player_Pawn.Player_Pawn_C|GetWepon_List _asplayer_pawn) self)
      (Transformation|AttachComponentToComponent (Variables|/Script/Engine.Character|GetMesh _asplayer_pawn) "wepon_2" "SnapToTarget" "SnapToTarget" "SnapToTarget" true)
      (Variables|Default|SetPickUp_frag true))))

(event EventBeginPlay)

(event Collision|EventActorBeginOverlap
  (params (OtherActor :type Actor%20Object%20Reference)))

(event EventTick
  (params (DeltaSeconds :type Float%20%28single-precision%29)))

(fn ConstructionScript)