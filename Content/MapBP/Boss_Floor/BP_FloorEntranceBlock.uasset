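; Boss-floor entrance blocker that shuts behind the player and reopens when the player dies.
; It starts with the blocking collision off and caches the player pawn.
; When the player stops overlapping the trigger, a DoOnce enables the blocker and disables the trigger.
; Tick polls the player's HP from the Status map, and at zero or below restores both collisions and resets the DoOnce.
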(event OnComponentEndOverlap(Disable_EntranceBlock_Collision)
  (params (OverlappedComponent :type Primitive%20Component%20Object%20Reference) (OtherActor :type Actor%20Object%20Reference) (OtherComp :type Primitive%20Component%20Object%20Reference) (OtherBodyIndex :type Integer))
  (Utilities|Casting|CastToPlayer_Pawn OtherActor)
  (Utilities|FlowControl|DoOnce false
    (:Completed
      (Collision|SetCollisionEnabled (Variables|Default|GetEnable_EntranceBlock_Collision) "QueryAndPhysics")
      (Collision|SetCollisionEnabled (Variables|Default|GetDisable_EntranceBlock_Collision) "NoCollision"))))

(event Custom|RssetCollision
  (Utilities|FlowControl|DoOnce false) ; enters at Reset
)

(event EventBeginPlay
  (Collision|SetCollisionEnabled (Variables|Default|GetEnable_EntranceBlock_Collision) "NoCollision")
  (bind _asplayer_pawn (Utilities|Casting|CastToPlayer_Pawn (Game|Player|GetPlayerPawn 0)))
  (Utilities|IsValid _asplayer_pawn
    (:Is%20Valid
      (Variables|Default|SetAs%20Player%20Pawn _asplayer_pawn))))

(event Collision|EventActorBeginOverlap
  (params (OtherActor :type Actor%20Object%20Reference)))

(event EventTick
  (params (DeltaSeconds :type Float%20%28single-precision%29))
  (if (<= (.Value (Utilities|Map|Find (Variables|/Game/Player/Blueprint/Player_Pawn.Player_Pawn_C|GetStatus (Variables|Default|GetAs%20Player%20Pawn)) "HP")) 0.0)
    (Collision|SetCollisionEnabled (Variables|Default|GetEnable_EntranceBlock_Collision) "NoCollision")
    (Collision|SetCollisionEnabled (Variables|Default|GetDisable_EntranceBlock_Collision) "QueryAndPhysics")
    (CallFunction|RssetCollision)))

(fn ConstructionScript)