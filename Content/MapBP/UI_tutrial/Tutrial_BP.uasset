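; Tutorial trigger actor that shows a TutrialScene widget when an actor tagged "Player" enters its Box and pauses the game.
; BeginPlay pre-creates the widget and enables input on the actor for player 0.
; Once triggered, pressing Enter unpauses, removes the widget and destroys the actor, so each tutorial appears only once.
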(event OnComponentBeginOverlap(Box)
  (params (OverlappedComponent :type Primitive%20Component%20Object%20Reference) (OtherActor :type Actor%20Object%20Reference) (OtherComp :type Primitive%20Component%20Object%20Reference) (OtherBodyIndex :type Integer) (bFromSweep :type Boolean) (SweepResult :type Hit%20Result%20Structure%20%28by%20ref%29))
  (if (Actor|ActorHasTag OtherActor "Player")
    (UserInterface|Viewport|AddtoViewport (Variables|Default|GetTutrial_UI) 0)
    (Game|SetGamePaused true)
    (Variables|Default|SetIN_Player true)))

(event EventBeginPlay
  (bind _returnvalue (UserInterface|CreateWidget (Variables|Default|GetTutrial_Scene) (Game|GetPlayerController 0)))
  (Variables|Default|SetTutrial_UI _returnvalue)
  (Input|EnableInput (Game|GetPlayerController 0)))

(event Collision|EventActorBeginOverlap
  (params (OtherActor :type Actor%20Object%20Reference)))

(event EventTick
  (params (DeltaSeconds :type Float%20%28single-precision%29)))

(event Input|KeyboardEvents|Enter
  (params (Key :type Key%20Structure :default "None"))
  (:Pressed
    (if (Variables|Default|GetIN_Player)
      (Game|SetGamePaused false)
      (Widget|RemovefromParent (Variables|Default|GetTutrial_UI))
      (Actor|DestroyActor))))

(fn ConstructionScript)