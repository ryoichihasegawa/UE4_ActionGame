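; BP_Magic is the enemy wizard's magic shot, which damages the player on contact.
; On spawn it plays a sound and takes the first BP_EnemyCharacter_Wizard_Base found in the world, not necessarily its shooter, as the damage source.
; Overlapping a "Body" component damages Player_Pawn, plays hit effects and destroys the shot.
; Map or wall overlaps destroy it only once the CoolTime countdown in Tick has expired.
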(event OnComponentBeginOverlap(Collision)
  (params (OverlappedComponent :type Primitive%20Component%20Object%20Reference) (OtherActor :type Actor%20Object%20Reference) (OtherComp :type Primitive%20Component%20Object%20Reference) (OtherBodyIndex :type Integer) (bFromSweep :type Boolean) (SweepResult :type Hit%20Result%20Structure%20%28by%20ref%29))
  (if (Components|ComponentHasTag OtherComp "Body")
    ;[1 1 1] playerのダメージ処理
    (bind _asplayer_pawn (Utilities|Casting|CastToPlayer_Pawn OtherActor))
    (Default|OnDamageEvent _asplayer_pawn _asplayer_pawn (Utilities|Struct|MakeDamage_Parameter (Variables|/Game/Enemy/Enemy_base.Enemy_base_C|GetEnemy_Damage%20Value (Variables|Default|GetEnemyWizard))))
    (Audio|PlaySound2D "/Game/Enemy/Sound/Magic/SC_MagicHit.SC_MagicHit" 1.0 1.0 0.0 0 0)
    (Effects|SpawnEmitteratLocation "/Game/FXVarietyPack/Particles/P_ky_waterBallHit.P_ky_waterBallHit" (Transformation|GetActorLocation OtherActor) "0, 0, 0" "0.500000,0.500000,0.500000")
    (Actor|DestroyActor)
    (elif (and (Math|Boolean|ORBoolean (Actor|ActorHasTag OtherActor "Map") (Components|ComponentHasTag OtherComp "Map") (Components|ComponentHasTag OtherComp "MapWall")) (<= (Variables|Default|GetCoolTime) 0.0))
      (Actor|DestroyActor))))

(event EventBeginPlay
  (bind _returnvalue (Actor|GetActorOfClass "/Game/Enemy/Character/Wizard_Base/BP_EnemyCharacter_Wizard_Base.BP_EnemyCharacter_Wizard_Base_C"))
  (Variables|Default|SetEnemyWizard _returnvalue)
  (Audio|PlaySound2D "/Game/Enemy/Sound/Magic/SC_MagicShot.SC_MagicShot" 1.0 1.0 0.0 0 0))

(event EventTick
  (params (DeltaSeconds :type Float%20%28single-precision%29))
  (if (>= (Variables|Default|GetCoolTime) 0.0)
    (Variables|Default|SetCoolTime (- (Variables|Default|GetCoolTime) DeltaSeconds))))

(fn ConstructionScript)