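; BP_ShadowActor is an enemy shadow skeletal-mesh actor whose opacity fades out over time.
; The construction script creates a dynamic material instance on the mesh.
; Init sets the Opa parameter and unhides the actor, and Tick lowers Opa by delta seconds while the active flag is set.
; Finish hides the actor and clears the flag, while nothing here stops the fade automatically at zero.
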(event Custom|Init
  (params (Opa :type Float%20%28single-precision%29))
  (Rendering|Material|SetScalarParameterValue (Variables|Default|GetShadowMaterial) "Opa" Opa :!class /Script/Engine.MaterialInstanceDynamic)
  (if (not (Variables|Default|GetFlag))
    (Rendering|SetActorHiddenInGame false)
    (Variables|Default|SetFlag true)))

(event Custom|Finish
  (Rendering|SetActorHiddenInGame true)
  (Variables|Default|SetFlag false))

(event EventTick
  (params (DeltaSeconds :type Float%20%28single-precision%29))
  (bind _shadowmaterial (Variables|Default|GetShadowMaterial))
  (if (Variables|Default|GetFlag)
    (bind _returnvalue (Rendering|Material|GetScalarParameterValue _shadowmaterial "Opa" :!class /Script/Engine.MaterialInstanceDynamic))
    (Rendering|Material|SetScalarParameterValue _shadowmaterial "Opa" (- _returnvalue DeltaSeconds) :!class /Script/Engine.MaterialInstanceDynamic)))

(fn ConstructionScript
  (bind _returnvalue (Rendering|Material|CreateDynamicMaterialInstance (Variables|Default|GetSkeletalMesh) 0 0 "None" :!class /Script/Engine.PrimitiveComponent))
  (Variables|Default|SetShadowMaterial _returnvalue))