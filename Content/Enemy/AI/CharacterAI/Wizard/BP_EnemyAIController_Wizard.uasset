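; AI controller for the Wizard enemy that starts its behavior tree on BeginPlay.
; Custom events act as setters that write values into Blackboard keys, referenced through key-name variables.
; These cover the target actor, line of sight, attack flag, random rolls for attack and warp, and cooldown times for both, feeding the tree's decisions.
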(event EventBeginPlay
  ;[1 1 1] 始まったら
  (AI|RunBehaviorTree (Variables|ビヘイビアツリー|GetBTAsset)))

(event EventUpdateHasLineOfSightKey
  (params (HasLineOfSight :type Boolean))
  ;[1 1 1 1 48] ブラックボードキーに格納
  ;;[1 0 0] Has Line Of Sight Keyをブラックボードに格納
  (AI|Components|Blackboard|SetValueasBool (Variables|Default|GetBlackboard) (Variables|BrackBoardKey|GetHasLineOfSightName) HasLineOfSight))

(event EventUpdateWarpCoolDownTimeKey
  (params (WarpCoolDownTime :type Float%20%28single-precision%29))
  ;[1 1 1 1 48] ブラックボードキーに格納
  ;;[0.2664 1 0.2031] ワープのクールダウンタイムをブラックボードに格納
  (AI|Components|Blackboard|SetValueasFloat (Variables|Default|GetBlackboard) (Variables|BrackBoardKey|GetWarpCoolDownTimeName) WarpCoolDownTime))

(event EventUpdateEnemyAttackFlagKey
  (params (EnemyAttackFlag :type Boolean))
  ;[1 1 1 1 48] ブラックボードキーに格納
  ;;[1 0 0] EnemyAttackFlagKey をブラックボードに格納
  (AI|Components|Blackboard|SetValueasBool (Variables|Default|GetBlackboard) (Variables|BrackBoardKey|GetEnemyAttackFlagName) EnemyAttackFlag))

(event EventUpdateTagetActorKey
  (params (TagetActor :type Actor%20Object%20Reference))
  ;[1 1 1 1 48] ブラックボードキーに格納
  ;;[0.5 0.5 1] Taget Actor Keyをブラックボードに格納
  (AI|Components|Blackboard|SetValueasObject (Variables|Default|GetBlackboard) (Variables|BrackBoardKey|GetTagetActorName) TagetActor))

(event EventUpdateAttackRandomKey
  (params (AttackRandam :type Float%20%28single-precision%29))
  ;[1 1 1 1 48] ブラックボードキーに格納
  ;;[0.2664 1 0.2031] AttackRandamをブラックボードに格納
  (AI|Components|Blackboard|SetValueasFloat (Variables|Default|GetBlackboard) (Variables|BrackBoardKey|GetAttackRandamName) AttackRandam))

(event EventUpdateWarpRandamKey
  (params (WarpRandam :type Float%20%28single-precision%29))
  ;[1 1 1 1 48] ブラックボードキーに格納
  ;;[0.2664 1 0.2031] WarpRandamをブラックボードに格納
  (AI|Components|Blackboard|SetValueasFloat (Variables|Default|GetBlackboard) (Variables|BrackBoardKey|GetWarpRandamName) WarpRandam))

(event EventUpdateAttackCoolDownTimeKey
  (params (AttackCoolDownTime :type Float%20%28single-precision%29))
  ;[1 1 1 1 48] ブラックボードキーに格納
  ;;[0.2664 1 0.2031] 攻撃のクールダウンタイムをブラックボードに格納
  (AI|Components|Blackboard|SetValueasFloat (Variables|Default|GetBlackboard) (Variables|BrackBoardKey|GetAttackCoolDownTimeName) AttackCoolDownTime))

(fn ConstructionScript)