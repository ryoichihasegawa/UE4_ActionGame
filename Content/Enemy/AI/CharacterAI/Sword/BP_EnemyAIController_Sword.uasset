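; AI controller for the sword enemy, which runs its behavior tree on BeginPlay.
; Custom events act as setters that write values into Blackboard keys through key-name variables.
; The keys cover player and target actors, line of sight, player attack and parry success flags, and random values and cooldown times for attack and avoidance.
; The controller itself makes no decisions beyond starting the tree and storing these values.
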(event EventBeginPlay
  ;[1 1 1] 始まったら
  (AI|RunBehaviorTree (Variables|ビヘイビアツリー|GetBTAsset)))

(event EventUpdateHasLineOfSightKey
  (params (HasLineOfSight :type Boolean))
  ;[1 1 1 1 48] ブラックボードキーに格納
  ;;[1 0 0] Has line of sight keyをブラックボードに格納
  (AI|Components|Blackboard|SetValueasBool (Variables|Default|GetBlackboard) (Variables|BrackBoardKey|GetHasLineOfSightName) HasLineOfSight))

(event EventUpdatePlayerAttackFlagKey
  (params (PlayerAttackFlag :type Boolean))
  ;[1 1 1 1 48] ブラックボードキーに格納
  ;;[1 0 0] PlayerAttackFlagをブラックボードに格納
  (AI|Components|Blackboard|SetValueasBool (Variables|Default|GetBlackboard) (Variables|BrackBoardKey|GetPlayerAttackFlagName) PlayerAttackFlag))

(event EventUpdateParrySuccessFlagKey
  (params (ParrySuccessFlag :type Boolean))
  ;[1 1 1 1 48] ブラックボードキーに格納
  ;;[1 0 0] ParrySuccessFlagをブラックボードに格納
  (AI|Components|Blackboard|SetValueasBool (Variables|Default|GetBlackboard) (Variables|BrackBoardKey|GetParrySuccessFlagName) ParrySuccessFlag))

(event EventUpdateTagetActorKey
  (params (TagetActor :type Actor%20Object%20Reference))
  ;[1 1 1 1 48] ブラックボードキーに格納
  ;;[0.5 0.5 1] Taget Actorをブラックボードに格納
  (AI|Components|Blackboard|SetValueasObject (Variables|Default|GetBlackboard) (Variables|BrackBoardKey|GetTagetActorName) TagetActor))

(event EventUpdateAvoidanceRandamKey
  (params (AvoidanceRandam :type Float%20%28single-precision%29))
  ;[1 1 1 1 48] ブラックボードキーに格納
  ;;[0.2664 1 0.2031] AvoidanceRandamをブラックボードに格納
  (AI|Components|Blackboard|SetValueasFloat (Variables|Default|GetBlackboard) (Variables|BrackBoardKey|GetAvoidanceRandamName) AvoidanceRandam))

(event EventUpdateAttackRandomKey
  (params (AttackRandam :type Float%20%28single-precision%29))
  ;[1 1 1 1 48] ブラックボードキーに格納
  ;;[0.2628 1 0.2021] AttackRandamをブラックボードに格納
  (AI|Components|Blackboard|SetValueasFloat (Variables|Default|GetBlackboard) (Variables|BrackBoardKey|GetAttackRandamName) AttackRandam))

(event EventUpdatePlayerActorKey
  (params (PlayerActor :type Actor%20Object%20Reference))
  ;[1 1 1 1 48] ブラックボードキーに格納
  ;;[0.5 0.5 1] Player Actorをブラックボードに格納
  (AI|Components|Blackboard|SetValueasObject (Variables|Default|GetBlackboard) (Variables|BrackBoardKey|GetPlayer%20Actor%20Name) PlayerActor))

(event EventUpdateAvoidanceCoolDownTimeKey
  (params (AvoidanceCoolDown :type Float%20%28single-precision%29))
  ;[1 1 1 1 48] ブラックボードキーに格納
  ;;[0.2637 1 0.2022] 回避のクールダウンタイムをブラックボードに格納
  (AI|Components|Blackboard|SetValueasFloat (Variables|Default|GetBlackboard) (Variables|BrackBoardKey|GetAvoidanceCoolDownTimeName) AvoidanceCoolDown))

(event EventUpdateAttackCoolDownTimeKey
  (params (AttackCoolDownTime :type Float%20%28single-precision%29))
  ;[1 1 1 1 48] ブラックボードキーに格納
  ;;[0.2628 1 0.2021] 攻撃のクールダウンタイムをブラックボードに格納
  (AI|Components|Blackboard|SetValueasFloat (Variables|Default|GetBlackboard) (Variables|BrackBoardKey|GetAttackCoolDownTimeName) AttackCoolDownTime))

(fn ConstructionScript)