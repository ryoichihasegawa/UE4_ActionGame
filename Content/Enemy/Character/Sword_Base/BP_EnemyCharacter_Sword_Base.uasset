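; Base sword enemy character that detects, attacks and dodges the player, and can be parried or ragdolled on death.
; AIPerception sets the target, alerts actors sharing its tag and clears the target after a timed sight loss.
; Tick pushes combat flags and cooldowns to the AIController as key messages.
; Attacks vary by distance and strength flag, timelines drive dash and dodge movement, and discovery or parry montages briefly pause brain logic.
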(event OnTargetPerceptionUpdated(AIPerception)
  (params (Actor :type Actor%20Object%20Reference) (Stimulus :type AI%20Stimulus%20Structure))
  (bind _aicontroller (Variables|Actor|GetAIController))
  (bind _aicontroller_2 (Variables|Actor|GetAIController))
  (bind _braincomponent (Variables|/Script/AIModule.AIController|GetBrainComponent _aicontroller))
  ;[0 1 0] AIPerception
  (Variables|Actor|SetPerceivedActor Actor)
  (if (and (== (Variables|Actor|GetPerceivedActor) (Variables|Actor|GetPlayerCharacter)) (Utilities|Struct|BreakAIStimulus Stimulus))
    (Variables|Actor|SetPerceivedActor (Variables|Actor|GetPlayerCharacter))
    (Utilities|FlowControl|Sequence
      (:then_0
        (Utilities|Time|ClearandInvalidateTimerbyHandle (Variables|AI|GetTagetLostTime))
        (Class|BPEnemyAIConInterface|UpdateTagetActorKey(Message) _aicontroller_2 (Variables|Actor|GetPerceivedActor))
        (Class|BPEnemyAIConInterface|UpdateHasLineOfSightKey(Message) _aicontroller_2 true)
        (Utilities|FlowControl|DoOnce false
          (:Completed
            (Components|Movement|StopMovementImmediately (Variables|Character|GetCharacterMovement))
            (AI|Logic|StopLogic _braincomponent "")
            (Animation|Montage|PlayMontage (Variables|Character|GetMesh) (Variables|発見|GetDiscoverAnim%20Montage)
              (:then
                (Utilities|FlowControl|Delay 1.0)
                (Class|BrainComponent|RestartLogic _braincomponent)
                (CallFunction|UpdateWalkSpeed (Variables|移動|GetDiscoverWalk%20Speed)) ; WalkSpeedを更新
              )))))
      (:then_1
        (bind _outactors (Actor|GetAllActorswithTag (Utilities|Array|Get(acopy) (Variables|Default|GetTags) 1)))
        (for _array_element _outactors
          (Class|BPEnemyAIConInterface|UpdateTagetActorKey(Message) (AI|GetAIController _array_element) (Variables|Actor|GetPerceivedActor)))))
    (elif (== (Variables|Actor|GetPlayerCharacter) (Variables|Actor|GetPerceivedActor))
      (bind _returnvalue (Utilities|Time|SetTimerbyEvent (delegate Custom|TagetLost) 5.0))
      (Variables|AI|SetTagetLostTime _returnvalue)
      (Class|BPEnemyAIConInterface|UpdateHasLineOfSightKey(Message) (Variables|Actor|GetAIController) false))))

(event Custom|Parry
  (bind _aicontroller (Variables|Actor|GetAIController))
  (bind _braincomponent (Variables|/Script/AIModule.AIController|GetBrainComponent _aicontroller))
  ;[1 1 1] パリィ処理
  (Variables|パリィ|SetParrySuccessFlag true)
  (AI|Logic|StopLogic _braincomponent "")
  (Collision|SetCollisionEnabled (Variables|Default|GetEnemy_Attack_1) "NoCollision")
  (Animation|StopAnimMontage (Variables|攻撃|GetAttackAnim%20Montage))
  (Animation|Montage|PlayMontage (Variables|Character|GetMesh) (Variables|パリィ|GetParryAnim%20Montage) (Variables|パリィ|GetParry%20Anim%20Play%20Rate)
    (:then
      (Variables|パリィ|SetParyTrueFrag false)
      (Utilities|FlowControl|Delay 3.0)
      (Class|BrainComponent|RestartLogic _braincomponent))
    (:OnCompleted
      (Variables|パリィ|SetParrySuccessFlag false :!label _label))
    (:OnInterrupted
      (goto _label))))

(event Custom|TagetLost
  (bind _aicontroller (Variables|Actor|GetAIController))
  (bind _braincomponent (Variables|/Script/AIModule.AIController|GetBrainComponent _aicontroller))
  ;[0 1 0] AIPerception
  (Class|BPEnemyAIConInterface|UpdateTagetActorKey(Message) (Variables|Actor|GetAIController))
  (AI|ClearFocus (Variables|Actor|GetAIController))
  (Utilities|FlowControl|DoOnce false) ; enters at Reset
)

(event EventBeginPlay
  (CallFunction|EnemyBegin self))

(event EventAvoidance
  ;[1 1 1] 回避処理
  (Animation|Montage|PlayMontage (Variables|Character|GetMesh) (Variables|回避|GetAvoidanceAnim%20Montage) (Variables|回避|GetAvoidance%20Anim%20Play%20Rate)
    (:then
      (Timeline|AvoidanceMoveTimeLine PlayFromStart
        (:Update
          (Transformation|SetActorLocation (CallFunction|ForwardMoveto self (Variables|回避|GetAvoidance%20Moving%20Distance)) true true)
          (Variables|回避|SetAvoidance%20Cool%20Down%20Time (Variables|回避|GetAvoidance%20Cool%20Down%20Initial%20Time)))))))

(event EventSetAvoidanceCoolDownTime
  ;[1 1 1] 回避処理
  (Class|BPEnemyAIConInterface|UpdateAvoidanceCoolDownTimeKey(Message) (Variables|Actor|GetAIController) (Variables|回避|GetAvoidance%20Cool%20Down%20Time)))

(event EventSetAttackCoolDownTime
  ;[1 1 1] 攻撃
  ;;[1 0 0] 攻撃処理
  ;;;[0 1 0] 攻撃のクールダウン時間を更新
  (Class|BPEnemyAIConInterface|UpdateAttackCoolDownTimeKey(Message) (Variables|Actor|GetAIController) (Variables|攻撃|GetAttack%20Cool%20Down%20Time)))

(event EventEnemyDamageDisable
  ;[1 1 1] 攻撃
  ;;[1 0.9658 0] 攻撃判定を呼び出し
  (|CallParentFunction)
  (Variables|攻撃|SetEnemyAttack%20Frag false))

(event EventAttack
  (bind _playercharacter (Variables|Actor|GetPlayerCharacter))
  (bind _return (CallFunction|ActorDistance _playercharacter))
  ;[1 1 1] 攻撃
  ;;[1 0 0] 攻撃処理
  (AI|ClearFocus (Variables|Actor|GetAIController)) ; 見続けるのをやめる
  (if (<= _return 3e+02) ; 距離300以内にいるか？
    (if (Variables|Default|GetStrengthEnemyFlag) ; 強いエネミーか？
      (if (Math|Random|RandomBool)
        (Animation|PlayAnimMontage (Variables|攻撃|GetAttackAnim%20Montage) (Variables|攻撃|GetAttack3%20Play%20Rate) "Anim_Attack3") ; 突き攻撃
        (else
          (Animation|PlayAnimMontage (Variables|攻撃|GetAttackAnim%20Montage) (Variables|攻撃|GetAttack%20Play%20Rate) (Variables|攻撃|GetAM_SectionAttackName) :!label _label) ; 普通攻撃
        ))
      (else
        (goto _label)))
    (Variables|攻撃|SetAttack%20Cool%20Down%20Time (Variables|攻撃|GetAttack%20Cool%20Down%20Initial%20Time) :!label _label_2) ; 全体のクールタイム
    (elif (<= _return 5e+02) ; 距離500以内にいるか？
      (Animation|Montage|PlayMontage (Variables|Character|GetMesh) (Variables|攻撃|GetAttackAnim%20Montage) (Variables|攻撃|GetAttack2%20Play%20Rate) 0.0 "Anim_Attack2" ; ダッシュ攻撃
        (:then
          (Timeline|AttackMoveTimeLine PlayFromStart ; アニメーションしながら移動
            (:Update
              (Transformation|SetActorLocation (CallFunction|ForwardMoveto self (Variables|攻撃|GetAttack2%20Moving%20Distance)) true true) ; 移動
              (Utilities|FlowControl|Delay (Variables|攻撃|GetAttack2RecastTime)) ; 攻撃した後の隙
              (goto _label_2))))))))

(event EventTick
  (params (DeltaSeconds :type Float%20%28single-precision%29))
  (bind _playercharacter (Variables|Actor|GetPlayerCharacter))
  (bind _asplayer_pawn (Utilities|Casting|CastToPlayer_Pawn _playercharacter))
  ;[1 1 1] 常にやる
  (bind _output_get (Variables|Default|SetTime DeltaSeconds))
  (|CallParentFunction _output_get)
  (Utilities|FlowControl|Sequence
    (:then_0
      (if (== (Variables|Actor|GetPlayerCharacter) (Variables|Actor|GetPerceivedActor))
        (AI|FocusPlayerUpdateKey _asplayer_pawn) ; Key更新
        (else
          (CallFunction|UpdateKey))))
    (:then_1
      ;;[1 0 0] パリィされた時の処理
      (if (and (Variables|/Game/Player/Blueprint/Player_Pawn.Player_Pawn_C|GetPary_Frag _asplayer_pawn) (Variables|パリィ|GetParyTrueFrag))
        (CallFunction|Parry) ; パリィ
      ))
    (:then_2
      ;;[0 0 1] CoolDownTime処理
      (Utilities|FlowControl|Sequence
        (:then_0
          (if (>= (Variables|攻撃|GetAttack%20Cool%20Down%20Time) 0.0)
            (bind _output_get_2 (Variables|攻撃|SetAttack%20Cool%20Down%20Time (- (Variables|攻撃|GetAttack%20Cool%20Down%20Time) (Variables|Default|GetTime))))
            (Class|BPEnemyAIConInterface|UpdateAttackCoolDownTimeKey(Message) (Variables|Actor|GetAIController) _output_get_2)))
        (:then_1
          (if (>= (Variables|回避|GetAvoidance%20Cool%20Down%20Time) 0.0)
            (bind _output_get_3 (Variables|回避|SetAvoidance%20Cool%20Down%20Time (- (Variables|回避|GetAvoidance%20Cool%20Down%20Time) (Variables|Default|GetTime))))
            (Class|BPEnemyAIConInterface|UpdateAvoidanceCoolDownTimeKey(Message) (Variables|Actor|GetAIController) _output_get_3)))))))

(event EventOnEnemyDamageEvent
  (params (In_Other_Actor :type Actor%20Object%20Reference) (Damage_Parameter :type Damage%20Parameter%20Structure))
  ;[1 1 1] ダメージ処理
  ;;[1 0 0] ダメージ食らった時の処理
  (|CallParentFunction In_Other_Actor Damage_Parameter))

(event EventMove
  (params (Location :type Vector :default "0, 0, 0"))
  (bind _aicontroller (Variables|Actor|GetAIController))
  ;[1 1 1] 移動処理
  (CallFunction|UpdateWalkSpeed 4e+02) ; WalkSpeedを更新
  (bind _return (CallFunction|IsAlive self))
  (if _return
    (AI|SetFocus _aicontroller (Variables|Actor|GetPlayerCharacter))
    (AI|Navigation|MovetoLocation (Variables|Actor|GetAIController) Location 5e+01 true true true true 0)
    (else
      (AI|ClearFocus _aicontroller))))

(event EventEndPlay
  (params (EndPlayReason :type EEndPlayReason%20Enum :default "Destroyed"))
  (|CallParentFunction EndPlayReason))

(event EventEnemyDamageEnable
  ;[1 1 1] 攻撃
  ;;[1 0.9658 0] 攻撃判定を呼び出し
  (|CallParentFunction)
  (Variables|攻撃|SetEnemyAttack%20Frag true))

(event EventHitAnimation
  (bind _aicontroller (Variables|Actor|GetAIController))
  ;[1 1 1] ダメージ処理
  ;;[0 1 0] 当たった時の処理
  (if (not (Variables|Default|GetStrengthEnemyFlag))
    (if (not (Variables|攻撃|GetEnemyAttack%20Frag))
      (Animation|PlayAnimMontage "/Game/Enemy/Animation/AnimationMontage/Corpse/AM_EnemyDamage.AM_EnemyDamage" 1.0 "None")
      (Audio|PlaySound2D "/Game/Enemy/Sound/Damage/SC_Damage.SC_Damage" 1.0 1.0 0.0 0 0)
      (bind _return (Class|BPEnemyInterface|IsAlive(Message) self))
      (if _return
        (AI|SetFocus _aicontroller (Variables|Actor|GetPlayerCharacter))
        (Variables|Actor|SetPerceivedActor (Variables|Actor|GetPlayerCharacter))
        (Class|BPEnemyAIConInterface|UpdateTagetActorKey(Message) (Variables|Actor|GetAIController) (Variables|Actor|GetPlayerCharacter))
        (else
          (AI|ClearFocus _aicontroller))))))

(event EventDeadAnimation
  (bind _mesh (Variables|Character|GetMesh))
  ;[1 1 1] ダメージ処理
  ;;[1 0 0.8039] 死亡処理
  (Audio|PlaySound2D "/Game/Enemy/Sound/Death/SC_Death.SC_Death" 1.0 1.0 0.0 0 0)
  (Class|SkeletalMeshComponent|SetAllBodiesSimulatePhysics _mesh true)
  (Collision|SetCollisionEnabled _mesh "PhysicsOnly")
  (Collision|SetCollisionEnabled (Variables|Default|GetEnemy_Attack_1) "NoCollision")
  (Effects|SpawnEmitteratLocation "/Game/StarterContent/Particles/P_Explosion.P_Explosion" (Transformation|GetActorLocation) "0, 0, 0" "0.700000,0.700000,0.700000"))

(fn ConstructionScript
  (|CallParentFunction))

(fn UpdateWalkSpeed
  (params (NewWalkSpeed :type Float%20%28single-precision%29))
  (Variables|/Script/Engine.CharacterMovementComponent|SetMaxWalkSpeed (Variables|Character|GetCharacterMovement) NewWalkSpeed))

(fn FocusPlayerUpdateKey
  (params (PlayerPawn :type Player%20Pawn%20Object%20Reference))
  (bind _aicontroller (Variables|Actor|GetAIController))
  ;[1 1 1] 常にプレイヤーのAttackFragを更新する
  (Class|BPEnemyAIConInterface|UpdatePlayerAttackFlagKey(Message) _aicontroller (Variables|/Game/Player/Blueprint/Player_Pawn.Player_Pawn_C|GetAttack_frag PlayerPawn))
  ;[1 1 1] パリィ成功したフラグを更新する
  (Class|BPEnemyAIConInterface|UpdateParrySuccessFlagKey(Message) _aicontroller (Variables|パリィ|GetParrySuccessFlag))
  ;[1 1 1] 攻撃の確率の値を更新
  (Class|BPEnemyAIConInterface|UpdateAttackRandomKey(Message) _aicontroller (Variables|AI|GetAttackRandam))
  ;[1 1 1] 回避の確率の値を更新
  (Class|BPEnemyAIConInterface|UpdateAvoidanceRandamKey(Message) _aicontroller (Variables|AI|GetAvoidanceRandam)))

(fn ActorDistance
  (params (TagetActor :type Actor%20Object%20Reference))
  (return (Math|Vector|VectorLengthXY (- (Transformation|GetActorLocation) (Transformation|GetActorLocation TagetActor)))))

(fn ForwardMoveto
  (params (Taget :type Actor%20Object%20Reference) (Moving%20distance :type Float%20%28single-precision%29))
  (return (+ (Transformation|GetActorLocation Taget) (* (Math|Vector|GetForwardVector (Variables|Default|GetCapsuleComponent)) Moving%20distance))))

(fn UpdateKey
  (bind _aicontroller (Variables|Actor|GetAIController))
  ;[1 1 1] 常にプレイヤーのAttackFragを更新する
  (Class|BPEnemyAIConInterface|UpdatePlayerAttackFlagKey(Message) _aicontroller false)
  ;[1 1 1] パリィ成功したフラグを更新する
  (Class|BPEnemyAIConInterface|UpdateParrySuccessFlagKey(Message) _aicontroller false)
  ;[1 1 1] 攻撃の確率の値を更新
  (Class|BPEnemyAIConInterface|UpdateAttackRandomKey(Message) _aicontroller (Variables|AI|GetAttackRandam))
  ;[1 1 1] 回避の確率の値を更新
  (Class|BPEnemyAIConInterface|UpdateAvoidanceRandamKey(Message) _aicontroller (Variables|AI|GetAvoidanceRandam)))

(fn EnemyBegin
  (|CallParentFunction)
  ;[1 1 1] 始まった瞬間に格納
  (Variables|Actor|SetPlayerCharacter (Game|GetPlayerCharacter 0))
  (Variables|Actor|SetAIController (AI|GetAIController self))
  ;[1 1 1] 初期値を格納
  (Variables|攻撃|SetAttack%20Cool%20Down%20Initial%20Time (Variables|攻撃|GetAttack%20Cool%20Down%20Time))
  (Variables|回避|SetAvoidance%20Cool%20Down%20Initial%20Time (Variables|回避|GetAvoidance%20Cool%20Down%20Time))
  ;[1 1 1] 始まったら更新する
  (Class|BPEnemyAIConInterface|UpdatePlayerActorKey(Message) (Variables|Actor|GetAIController) (Variables|Actor|GetPlayerCharacter))
  (Class|BPEnemyAIConInterface|UpdateAttackCoolDownTimeKey(Message) (Variables|Actor|GetAIController) 0.0)
  (Class|BPEnemyAIConInterface|UpdateAvoidanceCoolDownTimeKey(Message) (Variables|Actor|GetAIController) 0.0))

(fn IsAlive
  (return (> (Variables|Default|GetHP) 0.0)))