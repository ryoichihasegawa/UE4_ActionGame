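; BP_EnemyCharacter_Sword03 is a sword enemy character variant that customizes the hit reaction inherited from its parent Blueprint.
; Its HitAnimation event calls the parent, then spawns the NS_BasicHit effect at the mesh's upper spine socket and plays the SC_Damage sound in 2D.
; BeginPlay, overlap, Tick and the construction script add no logic of their own.
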(event EventBeginPlay
  (|CallParentFunction) ; このノードは無効になっているため呼び出せません。\n機能をビルドするにはピンをドラッグしてください。
)

(event Collision|EventActorBeginOverlap
  (params (OtherActor :type Actor%20Object%20Reference))
  (|CallParentFunction OtherActor) ; このノードは無効になっているため呼び出せません。\n機能をビルドするにはピンをドラッグしてください。
)

(event EventTick
  (params (DeltaSeconds :type Float%20%28single-precision%29))
  (|CallParentFunction DeltaSeconds) ; このノードは無効になっているため呼び出せません。\n機能をビルドするにはピンをドラッグしてください。
)

(event EventHitAnimation
  (|CallParentFunction)
  (Niagara|SpawnSystematLocation "/Game/EffectAssets/sA_Megapack_v1/sA_StylizedAttacksPack/FX/NiagaraSystems/NS_BasicHit.NS_BasicHit" (Transformation|GetSocketLocation (Variables|Character|GetMesh) "Bip001-Spine2"))
  (Audio|PlaySound2D "/Game/Enemy/Sound/Damage/SC_Damage.SC_Damage" 1.0 1.0 0.0 0 0))

(fn ConstructionScript
  (|CallParentFunction))